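; Planar lock joint part that toggles translational constraint between two attached bodies along the constraint's Y and Z axes.
; Locking sets both linear limits to Locked and wakes the joint base's rigid bodies, while unlocking sets them to Free.
; Repairing rebinds the physics constraint to the two bodies' root components, with the second body as the first component.
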(event EventBeginPlay
  (|CallParentFunction))

(event EventLockJoint
  (bind _jointconstraint (Variables|Default|GetJointConstraint))
  (Class|PhysicsConstraintComponent|SetLinearYLimit _jointconstraint "LCM_Locked" 0.0)
  (Class|PhysicsConstraintComponent|SetLinearZLimit _jointconstraint "LCM_Locked" 0.0)
  (Class|PrimitiveComponent|WakeAllRigidBodies (Variables|Default|GetJointBase)))

(event EventRepairJoint
  (Class|PhysicsConstraintComponent|SetConstrainedComponents (Variables|Default|GetJointConstraint) (Variables|/Game/InventorySystem/Items/Parts/BP_Body.BP_Body_C|GetBodyRoot (Utilities|Array|Get(acopy) (Variables|Default|GetBodies) 1)) "None" (Variables|/Game/InventorySystem/Items/Parts/BP_Body.BP_Body_C|GetBodyRoot (Utilities|Array|Get(acopy) (Variables|Default|GetBodies))) "None"))

(event EventUnlockJoint
  (bind _jointconstraint (Variables|Default|GetJointConstraint))
  (Class|PhysicsConstraintComponent|SetLinearYLimit _jointconstraint "LCM_Free" 0.0)
  (Class|PhysicsConstraintComponent|SetLinearZLimit _jointconstraint "LCM_Free" 0.0))

(fn ConstructionScript
  (|CallParentFunction))