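; BP_TestAxleTDiff is a test axle joint part, apparently a T-shaped differential, that links three physics bodies with constraints.
; RepairJoint re-binds X and Y constraints from bodies 1 and 2 to body 0, plus a transfer constraint between bodies 2 and 1.
; LockJoint and UnlockJoint switch only the X constraint's twist between locked and free; the matching Y calls are left disconnected.
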(event EventBeginPlay
  (|CallParentFunction))

(event EventRepairJoint
  (Development|PrintString "Repair Constraint" true true "(R=0.000000,G=0.660000,B=1.000000,A=1.000000)" 1e+02)
  (Class|PhysicsConstraintComponent|SetConstrainedComponents (Variables|Default|GetJointConstraintX) (Variables|/Game/InventorySystem/Items/Parts/BP_Body.BP_Body_C|GetBodyRoot (Utilities|Array|Get(acopy) (Variables|Default|GetBodies) 1)) "None" (Variables|/Game/InventorySystem/Items/Parts/BP_Body.BP_Body_C|GetBodyRoot (Utilities|Array|Get(acopy) (Variables|Default|GetBodies))) "None")
  (Class|PhysicsConstraintComponent|SetConstrainedComponents (Variables|Default|GetJointConstraintY) (Variables|/Game/InventorySystem/Items/Parts/BP_Body.BP_Body_C|GetBodyRoot (Utilities|Array|Get(acopy) (Variables|Default|GetBodies) 2)) "None" (Variables|/Game/InventorySystem/Items/Parts/BP_Body.BP_Body_C|GetBodyRoot (Utilities|Array|Get(acopy) (Variables|Default|GetBodies))) "None")
  (Class|PhysicsConstraintComponent|SetConstrainedComponents (Variables|Default|GetTransferConstraint) (Variables|/Game/InventorySystem/Items/Parts/BP_Body.BP_Body_C|GetBodyRoot (Utilities|Array|Get(acopy) (Variables|Default|GetBodies) 2)) "None" (Variables|/Game/InventorySystem/Items/Parts/BP_Body.BP_Body_C|GetBodyRoot (Utilities|Array|Get(acopy) (Variables|Default|GetBodies) 1)) "None"))

(event EventUnlockJoint
  (Class|PhysicsConstraintComponent|SetAngularTwistLimit (Variables|Default|GetJointConstraintX) "ACM_Free" 0.0))

(event EventLockJoint
  (Class|PhysicsConstraintComponent|SetAngularTwistLimit (Variables|Default|GetJointConstraintX) "ACM_Locked" 0.0))

(fn ConstructionScript
  (|CallParentFunction))