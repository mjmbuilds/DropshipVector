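; BP_TankTread is a tank tread joint part made of two track blocks and a physics constraint between bodies.
; LockJoint stiffens the angular drive toward a target angle and wakes the track, UnlockJoint zeroes its strength, and RepairJoint reconnects both body roots to the constraint.
; InitScale repurposes ScaleZ as an angle adjusting block rotation and constraint offset, while ScaleX and ScaleY resize both blocks at half rate with caps.
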(event EventBeginPlay
  (|CallParentFunction) ; This node is disabled and will not be called.\nDrag off pins to build functionality.
)

(event Collision|EventActorBeginOverlap
  (params (OtherActor :type Actor%20Object%20Reference)))

(event EventTick
  (params (DeltaSeconds :type Float%20%28single-precision%29))
  (|CallParentFunction DeltaSeconds))

(event EventLockJoint
  (bind _physicsconstraint (Variables|Default|GetPhysicsConstraint))
  (Class|PhysicsConstraintComponent|SetAngularOrientationTarget _physicsconstraint (Math|Rotator|MakeRotator (+ -45.0 (- (Variables|Default|GetScaleZ) 1.0)) 0.0 0.0))
  (Class|PhysicsConstraintComponent|SetAngularDriveParams _physicsconstraint 1e+10 1e+02 0.0)
  (Class|PrimitiveComponent|WakeAllRigidBodies (Variables|Default|GetTankTrackBlock1)))

(event EventUnlockJoint
  (Class|PhysicsConstraintComponent|SetAngularDriveParams (Variables|Default|GetPhysicsConstraint) 0.0 1e+02 0.0))

(event EventRepairJoint
  (Class|PhysicsConstraintComponent|SetConstrainedComponents (Variables|Default|GetPhysicsConstraint) (Variables|/Game/InventorySystem/Items/Parts/BP_Body.BP_Body_C|GetBodyRoot (Utilities|Array|Get(acopy) (Variables|Default|GetBodies) 1)) "None" (Variables|/Game/InventorySystem/Items/Parts/BP_Body.BP_Body_C|GetBodyRoot (Utilities|Array|Get(acopy) (Variables|Default|GetBodies))) "None"))

(event EventInitScale
  (bind _scalez (Variables|Default|GetScaleZ))
  (bind _scalex (Variables|Default|GetScaleX))
  (bind _scaley (Variables|Default|GetScaleY))
  (bind _returnvalue (- _scalez 1.0))
  (bind _returnvalue_2 (- _scalex 1.0))
  (bind _returnvalue_3 (- _scaley 1.0))
  (bind _returnvalue_4 (* _returnvalue_2 0.5))
  (bind _returnvalue_5 (* _returnvalue_3 0.5))
  (bind _returnvalue_6 (+ _returnvalue_4 1.0))
  (bind _returnvalue_7 (+ _returnvalue_5 1.0))
  (bind _returnvalue_8 (Math|Float|Min(Float) _returnvalue_6 3.0))
  (bind _returnvalue_9 (Math|Float|Min(Float) _returnvalue_7 5.0))
  (Transformation|AddLocalRotation (Variables|Default|GetTankTrackBlock2) (Math|Rotator|MakeRotator 0.0 _returnvalue 0.0) false false)
  (Class|CppFunctionLibrary|SetAngularRotationOffset (Variables|Default|GetPhysicsConstraint) 0.0 0.0 (- 45.0 _returnvalue))
  (Transformation|SetRelativeScale3D (Variables|Default|GetTankTrackBlock1) (Math|Vector|MakeVector _returnvalue_8 _returnvalue_9 1.0))
  (Transformation|SetRelativeScale3D (Variables|Default|GetTankTrackBlock2) (Math|Vector|MakeVector _returnvalue_8 _returnvalue_9 1.0)))

(fn ConstructionScript
  (|CallParentFunction))