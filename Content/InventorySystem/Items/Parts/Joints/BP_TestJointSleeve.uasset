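; BP_TestJointSleeve is a test sleeve joint part that constrains itself to whichever BP_Part sits along its axis.
; Outside build mode, each Tick traces from JointBase to Top and constrains the hit part's body to its own first body, breaking first when that body is unchanged.
; Missing a part breaks the constraint and clears the body.
; Lock, Unlock and Repair events lock or limit linear X travel, or re-attach the stored body.
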(event EventBeginPlay
  (|CallParentFunction))

(event EventUnlockJoint
  (Class|PhysicsConstraintComponent|SetLinearXLimit (Variables|Default|GetJointConstraint) "LCM_Limited" 4e+01))

(event EventRepairJoint
  (bind _constrainedbody (Variables|Default|GetConstrainedBody))
  (Development|PrintString "Repair Constraint" true true "(R=0.000000,G=0.660000,B=1.000000,A=1.000000)" 1e+02)
  (Utilities|IsValid _constrainedbody
    (:Is%20Valid
      (Class|PhysicsConstraintComponent|SetConstrainedComponents (Variables|Default|GetJointConstraint) (Variables|/Game/InventorySystem/Items/Parts/BP_Body.BP_Body_C|GetBodyRoot _constrainedbody) "None" (Variables|/Game/InventorySystem/Items/Parts/BP_Body.BP_Body_C|GetBodyRoot (Utilities|Array|Get(acopy) (Variables|Default|GetBodies))) "None"))))

(event EventTick
  (params (DeltaSeconds :type Float%20%28single-precision%29))
  (bind _jointconstraint (Variables|Default|GetJointConstraint))
  (if (not (Variables|Default|GetInBuildMode))
    (bind (_outhit _returnvalue) (Collision|LineTraceByChannel (Transformation|GetWorldLocation (Variables|Default|GetJointBase)) (Transformation|GetWorldLocation (Variables|Default|GetTop)) "TraceTypeQuery1" false 0 "None"))
    (if _returnvalue
      (Utilities|Casting|CastToBP_Part (.HitActor (Collision|BreakHitResult _outhit))
        (:then
          (Utilities|IsValid (Variables|Default|GetConstrainedBody)
            (:Is%20Valid
              (if (== (Variables|Default|GetConstrainedBody) (.Body (CallFunction|GetBodyfromComp (.HitComponent (Collision|BreakHitResult _outhit)))))
                (Class|PhysicsConstraintComponent|BreakConstraint (Variables|Default|GetJointConstraint))))
            (:Is%20Not%20Valid
              _))
          (bind _output_get (Variables|Default|SetConstrainedBody (.Body (CallFunction|GetBodyfromComp (.HitComponent (Collision|BreakHitResult _outhit))))))
          (Class|PhysicsConstraintComponent|SetConstrainedComponents _jointconstraint (Variables|/Game/InventorySystem/Items/Parts/BP_Body.BP_Body_C|GetBodyRoot _output_get) "None" (Variables|/Game/InventorySystem/Items/Parts/BP_Body.BP_Body_C|GetBodyRoot (Utilities|Array|Get(acopy) (Variables|Default|GetBodies))) "None")
          (Class|PhysicsConstraintComponent|SetConstraintReferencePosition _jointconstraint "Frame1" (Math|Vector|MakeVector 0.0 0.0 0.0)))
        (:CastFailed
          (Utilities|IsValid (Variables|Default|GetConstrainedBody) :!label _label
            (:Is%20Valid
              (Class|PhysicsConstraintComponent|BreakConstraint (Variables|Default|GetJointConstraint))
              (Variables|Default|SetConstrainedBody 0)))))
      (else
        (goto _label)))))

(event EventLockJoint
  (Class|PhysicsConstraintComponent|SetLinearXLimit (Variables|Default|GetJointConstraint) "LCM_Locked" 0.0))

(fn ConstructionScript
  (|CallParentFunction))