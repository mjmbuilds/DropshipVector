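; Test differential axle joint part in the inventory item system, built from physics constraints between four bodies.
; RepairJoint rebinds F, R and L joint constraints to the base body, plus two transfer constraints linking the F body to R and L.
; LockJoint and UnlockJoint toggle twist between locked and free on the F constraint only; matching R and L calls are left unwired.
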(event EventBeginPlay
  (|CallParentFunction))

(event EventRepairJoint
  (Development|PrintString "Repair Constraint" true true "(R=0.000000,G=0.660000,B=1.000000,A=1.000000)" 1e+02)
  (Class|PhysicsConstraintComponent|SetConstrainedComponents (Variables|Default|GetJointConstraintF) (Variables|/Game/InventorySystem/Items/Parts/BP_Body.BP_Body_C|GetBodyRoot (Utilities|Array|Get(acopy) (Variables|Default|GetBodies) 1)) "None" (Variables|/Game/InventorySystem/Items/Parts/BP_Body.BP_Body_C|GetBodyRoot (Utilities|Array|Get(acopy) (Variables|Default|GetBodies))) "None")
  (Class|PhysicsConstraintComponent|SetConstrainedComponents (Variables|Default|GetJointConstraintR) (Variables|/Game/InventorySystem/Items/Parts/BP_Body.BP_Body_C|GetBodyRoot (Utilities|Array|Get(acopy) (Variables|Default|GetBodies) 2)) "None" (Variables|/Game/InventorySystem/Items/Parts/BP_Body.BP_Body_C|GetBodyRoot (Utilities|Array|Get(acopy) (Variables|Default|GetBodies))) "None")
  (Class|PhysicsConstraintComponent|SetConstrainedComponents (Variables|Default|GetJointConstraintL) (Variables|/Game/InventorySystem/Items/Parts/BP_Body.BP_Body_C|GetBodyRoot (Utilities|Array|Get(acopy) (Variables|Default|GetBodies) 3)) "None" (Variables|/Game/InventorySystem/Items/Parts/BP_Body.BP_Body_C|GetBodyRoot (Utilities|Array|Get(acopy) (Variables|Default|GetBodies))) "None")
  (Class|PhysicsConstraintComponent|SetConstrainedComponents (Variables|Default|GetTransferConstraintFR) (Variables|/Game/InventorySystem/Items/Parts/BP_Body.BP_Body_C|GetBodyRoot (Utilities|Array|Get(acopy) (Variables|Default|GetBodies) 2)) "None" (Variables|/Game/InventorySystem/Items/Parts/BP_Body.BP_Body_C|GetBodyRoot (Utilities|Array|Get(acopy) (Variables|Default|GetBodies) 1)) "None")
  (Class|PhysicsConstraintComponent|SetConstrainedComponents (Variables|Default|GetTransferConstraintFL) (Variables|/Game/InventorySystem/Items/Parts/BP_Body.BP_Body_C|GetBodyRoot (Utilities|Array|Get(acopy) (Variables|Default|GetBodies) 3)) "None" (Variables|/Game/InventorySystem/Items/Parts/BP_Body.BP_Body_C|GetBodyRoot (Utilities|Array|Get(acopy) (Variables|Default|GetBodies) 1)) "None"))

(event EventUnlockJoint
  (Class|PhysicsConstraintComponent|SetAngularTwistLimit (Variables|Default|GetJointConstraintF) "ACM_Free" 0.0))

(event EventLockJoint
  (Class|PhysicsConstraintComponent|SetAngularTwistLimit (Variables|Default|GetJointConstraintF) "ACM_Locked" 0.0))

(fn ConstructionScript
  (|CallParentFunction))