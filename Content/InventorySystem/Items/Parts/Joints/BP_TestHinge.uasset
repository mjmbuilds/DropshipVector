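; BP_TestHinge is a test hinge joint part in the inventory item system that drives a physics constraint between two bodies.
; Unlock and lock events switch the constraint's angular Swing1 limit between a wide limited range and fully locked.
; The repair event prints a debug message, re-binds the constraint to the two bodies' roots and resets the first frame's reference orientation axes.
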(event EventBeginPlay
  (|CallParentFunction))

(event EventRepairJoint
  (Development|PrintString "Repair Constraint" true true "(R=0.000000,G=0.660000,B=1.000000,A=1.000000)" 1e+02)
  (Class|PhysicsConstraintComponent|SetConstrainedComponents (Variables|Default|GetJointConstraint) (Variables|/Game/InventorySystem/Items/Parts/BP_Body.BP_Body_C|GetBodyRoot (Utilities|Array|Get(acopy) (Variables|Default|GetBodies) 1)) "None" (Variables|/Game/InventorySystem/Items/Parts/BP_Body.BP_Body_C|GetBodyRoot (Utilities|Array|Get(acopy) (Variables|Default|GetBodies))) "None")
  (Class|PhysicsConstraintComponent|SetConstraintReferenceOrientation (Variables|Default|GetJointConstraint) "Frame1" (Math|Vector|MakeVector 1.0 0.0 0.0) (Math|Vector|MakeVector 0.0 1.0 0.0)))

(event EventUnlockJoint
  (Class|PhysicsConstraintComponent|SetAngularSwing1Limit (Variables|Default|GetJointConstraint) "ACM_Limited" 1.8e+02))

(event EventLockJoint
  (Class|PhysicsConstraintComponent|SetAngularSwing1Limit (Variables|Default|GetJointConstraint) "ACM_Locked" 0.0))

(fn ConstructionScript
  (|CallParentFunction))