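; BP_Suspension1 is a buildable suspension joint part that acts as a spring between two bodies through a physics constraint's linear drive.
; Events tune the spring, lock or free its Z travel, and repair the joint by reconnecting both bodies.
; Outside build mode, Tick stretches the spring's center component to the base-to-end distance and sharply overrides drive strength past a length threshold, otherwise using the configured strength.
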(event Custom|AdjustSpring
  (params (Strength :type Float%20%28single-precision%29) (Damping :type Float%20%28single-precision%29) (MaxForce :type Float%20%28single-precision%29))
  (bind _output_get (Variables|Default|SetSpringStrength Strength))
  (bind _output_get_2 (Variables|Default|SetSpringDamping Damping))
  (bind _output_get_3 (Variables|Default|SetSpringMaxForce MaxForce))
  (Class|PhysicsConstraintComponent|SetLinearDriveParams (Variables|Default|GetPhysicsConstraint) _output_get _output_get_2 _output_get_3))

(event EventBeginPlay
  (|CallParentFunction)
  (Class|PhysicsConstraintComponent|SetLinearDriveParams (Variables|Default|GetPhysicsConstraint) (Variables|Default|GetSpringStrength) (Variables|Default|GetSpringDamping) (Variables|Default|GetSpringMaxForce)))

(event EventTick
  (params (DeltaSeconds :type Float%20%28single-precision%29))
  (bind _springdamping (Variables|Default|GetSpringDamping))
  (bind _springmaxforce (Variables|Default|GetSpringMaxForce))
  (bind _spring1_base (Variables|Default|GetSpring1_Base))
  (bind _spring1_end (Variables|Default|GetSpring1_End))
  (bind _physicsconstraint (Variables|Default|GetPhysicsConstraint))
  (bind _returnvalue (Transformation|GetWorldLocation _spring1_base))
  (bind _returnvalue_2 (Transformation|GetWorldLocation _spring1_end))
  (bind _returnvalue_3 (- _returnvalue _returnvalue_2))
  (bind _returnvalue_4 (Math|Vector|VectorLength _returnvalue_3))
  (|CallParentFunction DeltaSeconds)
  (if (< (Variables|Default|GetDestroyTimer) 0)
    (Utilities|IsValid self
      (:Is%20Valid
        (if (not (Variables|Default|GetInBuildMode))
          (Transformation|SetRelativeScale3D (Variables|Default|GetSpring1_Center) (Math|Vector|MakeVector 1.0 1.0 _returnvalue_4))
          (if (> _returnvalue_4 2e+01)
            (Class|PhysicsConstraintComponent|SetLinearDriveParams _physicsconstraint 1e+05 _springdamping _springmaxforce)
            (else
              (Class|PhysicsConstraintComponent|SetLinearDriveParams _physicsconstraint (Variables|Default|GetSpringStrength) _springdamping _springmaxforce))))))))

(event EventLockJoint
  (Class|PhysicsConstraintComponent|SetLinearZLimit (Variables|Default|GetPhysicsConstraint) "LCM_Locked" 3e+02))

(event EventUnlockJoint
  (Class|PhysicsConstraintComponent|SetLinearZLimit (Variables|Default|GetPhysicsConstraint) "LCM_Limited" 3e+02))

(event EventRepairJoint
  (Class|PhysicsConstraintComponent|SetConstrainedComponents (Variables|Default|GetPhysicsConstraint) (Variables|/Game/InventorySystem/Items/Parts/BP_Body.BP_Body_C|GetBodyRoot (Utilities|Array|Get(acopy) (Variables|Default|GetBodies) 1)) "None" (Variables|/Game/InventorySystem/Items/Parts/BP_Body.BP_Body_C|GetBodyRoot (Utilities|Array|Get(acopy) (Variables|Default|GetBodies))) "None"))

(fn ConstructionScript
  (|CallParentFunction))