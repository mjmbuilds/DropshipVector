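; Test differential joint part that fakes a three-way gear differential between its joint ends using physics.
; Three constraints tie outer bodies to the first body, with events to lock or free their twist and to re-link them on repair.
; Outside build mode, Tick overwrites each end's angular velocity in sequence, mixing all three ends' velocities through 90- and 180-degree vector rotations instead of simulating gears.
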(event EventBeginPlay
  (|CallParentFunction))

(event EventTick
  (params (DeltaSeconds :type Float%20%28single-precision%29))
  (bind _jointend2 (Variables|Default|GetJointEnd2))
  (bind _jointend3 (Variables|Default|GetJointEnd3))
  (bind _jointend1 (Variables|Default|GetJointEnd1))
  (bind _returnvalue (Physics|GetPhysicsAngularVelocityinDegrees _jointend2 "None"))
  (bind _returnvalue_2 (Physics|GetPhysicsAngularVelocityinDegrees _jointend3 "None"))
  (bind _returnvalue_3 (Physics|GetPhysicsAngularVelocityinDegrees _jointend1 "None"))
  (bind _returnvalue_4 (Math|Vector|RotateVector _returnvalue_3 "0,90.000000, 0"))
  (bind _returnvalue_5 (Math|Vector|RotateVector _returnvalue_2 "0,180.000000, 0"))
  (bind _returnvalue_6 (+ _returnvalue _returnvalue_5))
  (bind _returnvalue_7 (/ _returnvalue_6 2.0))
  (|CallParentFunction DeltaSeconds)
  (if (not (Variables|Default|GetInBuildMode))
    (Class|PrimitiveComponent|SetAllPhysicsAngularVelocityinDegrees (Variables|Default|GetJointEnd2) (/ (+ _returnvalue_7 _returnvalue_4) 1.0) false)
    (Class|PrimitiveComponent|SetAllPhysicsAngularVelocityinDegrees (Variables|Default|GetJointEnd3) (/ (+ (Math|Vector|RotateVector _returnvalue_7 "0,180.000000, 0") _returnvalue_4) 1.0) false)
    (Class|PrimitiveComponent|SetAllPhysicsAngularVelocityinDegrees (Variables|Default|GetJointEnd1) (Math|Vector|RotateVector (/ (+ _returnvalue _returnvalue_2 _returnvalue_4) 3.0) "0,-90.000000, 0") false)))

(event EventRepairJoint
  (Development|PrintString "Repair Constraint" true true "(R=0.000000,G=0.660000,B=1.000000,A=1.000000)" 1e+02)
  (Class|PhysicsConstraintComponent|SetConstrainedComponents (Variables|Default|GetJointConstraint1) (Variables|/Game/InventorySystem/Items/Parts/BP_Body.BP_Body_C|GetBodyRoot (Utilities|Array|Get(acopy) (Variables|Default|GetBodies) 1)) "None" (Variables|/Game/InventorySystem/Items/Parts/BP_Body.BP_Body_C|GetBodyRoot (Utilities|Array|Get(acopy) (Variables|Default|GetBodies))) "None")
  (Class|PhysicsConstraintComponent|SetConstrainedComponents (Variables|Default|GetJointConstraint2) (Variables|/Game/InventorySystem/Items/Parts/BP_Body.BP_Body_C|GetBodyRoot (Utilities|Array|Get(acopy) (Variables|Default|GetBodies) 2)) "None" (Variables|/Game/InventorySystem/Items/Parts/BP_Body.BP_Body_C|GetBodyRoot (Utilities|Array|Get(acopy) (Variables|Default|GetBodies))) "None")
  (Class|PhysicsConstraintComponent|SetConstrainedComponents (Variables|Default|GetJointConstraint3) (Variables|/Game/InventorySystem/Items/Parts/BP_Body.BP_Body_C|GetBodyRoot (Utilities|Array|Get(acopy) (Variables|Default|GetBodies) 3)) "None" (Variables|/Game/InventorySystem/Items/Parts/BP_Body.BP_Body_C|GetBodyRoot (Utilities|Array|Get(acopy) (Variables|Default|GetBodies))) "None"))

(event EventUnlockJoint
  (Class|PhysicsConstraintComponent|SetAngularTwistLimit (Variables|Default|GetJointConstraint1) "ACM_Free" 0.0)
  (Class|PhysicsConstraintComponent|SetAngularTwistLimit (Variables|Default|GetJointConstraint2) "ACM_Free" 0.0)
  (Class|PhysicsConstraintComponent|SetAngularTwistLimit (Variables|Default|GetJointConstraint3) "ACM_Free" 0.0))

(event EventLockJoint
  (Class|PhysicsConstraintComponent|SetAngularTwistLimit (Variables|Default|GetJointConstraint1) "ACM_Locked" 0.0)
  (Class|PhysicsConstraintComponent|SetAngularTwistLimit (Variables|Default|GetJointConstraint2) "ACM_Locked" 0.0)
  (Class|PhysicsConstraintComponent|SetAngularTwistLimit (Variables|Default|GetJointConstraint3) "ACM_Locked" 0.0))

(fn ConstructionScript
  (|CallParentFunction))