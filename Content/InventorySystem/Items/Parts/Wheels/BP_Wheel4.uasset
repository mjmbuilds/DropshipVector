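; BP_Wheel4 is a wheel part Blueprint in the inventory system that currently adds on-screen physics debugging to its parent's behavior.
; Each Tick calls the parent, then prints Wheel1's linear velocity, velocity at a zero point, and angular velocity in radians and degrees.
; TrunkDelayVect slows the readout by caching truncated vectors per index, refreshing one slot whenever a countdown shared by all readouts expires.
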(event Collision|EventActorBeginOverlap
  (params (OtherActor :type Actor%20Object%20Reference)))

(event EventTick
  (params (DeltaSeconds :type Float%20%28single-precision%29))
  (bind _wheel1 (Variables|Default|GetWheel1))
  (|CallParentFunction DeltaSeconds)
  (bind _returnvalue (Physics|GetPhysicsLinearVelocity _wheel1 "None"))
  (bind _returnvalue_2 (Class|PrimitiveComponent|GetPhysicsLinearVelocityatPoint _wheel1 "0, 0, 0" "None"))
  (Development|PrintString (Utilities|String|Append "Lin Vel at P: " (CallFunction|TrunkDelayVect _returnvalue_2)) true true "(R=0.216164,G=1.000000,B=0.000000,A=1.000000)" 0.0)
  (Development|PrintString (Utilities|String|Append "Lin Vel: " (CallFunction|TrunkDelayVect _returnvalue 1)) true true "(R=0.216164,G=1.000000,B=0.000000,A=1.000000)" 0.0)
  (Development|PrintString (Utilities|String|Append "Ang Vel Rad: " (CallFunction|TrunkDelayVect (Class|PrimitiveComponent|GetPhysicsAngularVelocityinRadians _wheel1 "None") 2)) true true "(R=0.216164,G=1.000000,B=0.000000,A=1.000000)" 0.0)
  (Development|PrintString (Utilities|String|Append "Ang Vel Deg: " (CallFunction|TrunkDelayVect (Physics|GetPhysicsAngularVelocityinDegrees _wheel1 "None") 3)) true true "(R=0.216164,G=1.000000,B=0.000000,A=1.000000)" 0.0))

(fn ConstructionScript
  (|CallParentFunction))

(fn TrunkDelayVect
  (params (In :type Vector) (Index :type Integer))
  (if (<= (Variables|Default|GetDelayInt) 0)
    (Variables|Default|SetDelayInt 10) ; Delay
    (Utilities|Array|SetArrayElem (Variables|Default|GetDelayVects) Index (Math|Vector|MakeVector (Math|Conversions|ToFloat(Integer) (Math|Float|Truncate (.x In))) (Math|Conversions|ToFloat(Integer) (Math|Float|Truncate (.y In))) (Math|Conversions|ToFloat(Integer) (Math|Float|Truncate (.z In)))) true)
    (else
      (Math|Integer|DecrementInt (Variables|Default|GetDelayInt)
        (:%20%20
          _))))
  (return (Utilities|String|ToString(Vector) (Utilities|Array|Get(acopy) (Variables|Default|GetDelayVects) Index))))