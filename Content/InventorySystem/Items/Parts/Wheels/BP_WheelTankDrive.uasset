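; BP_WheelTankDrive is a tank drive wheel part in the inventory item system, built around a physics constraint between two bodies.
; Lock and unlock events toggle the constraint's linear X, linear Z and Swing2 motion between Locked and Free.
; A repair event re-links the constraint to the root components of the second and first entries in Bodies.
; The construction script only calls its parent, and BeginPlay, Tick and overlap are disabled stubs.
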(event EventBeginPlay
  (|CallParentFunction) ; This node is disabled and will not be called.\nDrag off pins to build functionality.
)

(event Collision|EventActorBeginOverlap
  (params (OtherActor :type Actor%20Object%20Reference)))

(event EventTick
  (params (DeltaSeconds :type Float%20%28single-precision%29))
  (|CallParentFunction DeltaSeconds) ; This node is disabled and will not be called.\nDrag off pins to build functionality.
)

(event EventLockJoint
  (bind _physicsconstraint (Variables|Default|GetPhysicsConstraint))
  (Class|PhysicsConstraintComponent|SetLinearXLimit _physicsconstraint "LCM_Locked" 0.0)
  (Class|PhysicsConstraintComponent|SetLinearZLimit _physicsconstraint "LCM_Locked" 0.0)
  (Class|PhysicsConstraintComponent|SetAngularSwing2Limit _physicsconstraint "ACM_Locked" 0.0))

(event EventUnlockJoint
  (bind _physicsconstraint (Variables|Default|GetPhysicsConstraint))
  (Class|PhysicsConstraintComponent|SetLinearXLimit _physicsconstraint "LCM_Free" 0.0)
  (Class|PhysicsConstraintComponent|SetLinearZLimit _physicsconstraint "LCM_Free" 0.0)
  (Class|PhysicsConstraintComponent|SetAngularSwing2Limit _physicsconstraint "ACM_Free" 0.0))

(event EventRepairJoint
  (Class|PhysicsConstraintComponent|SetConstrainedComponents (Variables|Default|GetPhysicsConstraint) (Variables|/Game/InventorySystem/Items/Parts/BP_Body.BP_Body_C|GetBodyRoot (Utilities|Array|Get(acopy) (Variables|Default|GetBodies) 1)) "None" (Variables|/Game/InventorySystem/Items/Parts/BP_Body.BP_Body_C|GetBodyRoot (Utilities|Array|Get(acopy) (Variables|Default|GetBodies))) "None"))

(fn ConstructionScript
  (|CallParentFunction))