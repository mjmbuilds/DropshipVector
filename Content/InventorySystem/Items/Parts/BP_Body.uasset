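; BP_Body is a physics body grouping connected part components under one root within a Creation, destroying itself when empty.
; It merges into other bodies, combining Creations as needed, and manages grounding, stasis, center of mass and wire nodes.
; After member removal, Tick triggers a neighbor flood-fill outside stasis that splits disconnected groups into new bodies.
; A crawl across joints then assigns those bodies to Creations, and wire nodes follow their parts.
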(event EventEndPlay
  (params (EndPlayReason :type EEndPlayReason%20Enum :default "Destroyed"))
  ;[1 1 1] Debug
  (Development|PrintString (Utilities|String|Append (Utilities|GetDisplayName self) " was Destroyed") (Variables|Default|GetDEBUG_Print) true "(R=0.000000,G=0.000000,B=0.500000,A=1.000000)" 1e+02))

(event EventTick
  (params (DeltaSeconds :type Float%20%28single-precision%29))
  (bind _creation (Variables|Default|GetCreation))
  (if (< (Utilities|Array|Length (Variables|Default|GetMembers)) 1)
    (if (not (Variables|Default|GetDisableDestroy))
      (Utilities|IsValid _creation
        (:Is%20Valid
          (Default|RemoveBody _creation self))
        (:Is%20Not%20Valid
          _))
      (Actor|DestroyActor))
    (elif (Variables|Default|GetNeedsRecalc)
      (if (not (Variables|/Game/InventorySystem/Items/Parts/BP_Creation.BP_Creation_C|GetInStasis (Variables|Default|GetCreation)))
        (CallFunction|RecalcBody)))))

(event EventBeginPlay
  (bind _creation (Variables|Default|GetCreation))
  ;[1 1 1] Debug
  (Development|PrintString (Utilities|String|Append (Utilities|GetDisplayName self) " Created") (Variables|Default|GetDEBUG_Print) true "(R=0.000000,G=0.000000,B=1.000000,A=1.000000)" 1e+02)
  (Utilities|IsValid _creation
    (:Is%20Valid
      (Default|AddBody _creation self))))

(fn ConstructionScript)

(fn MergeBodies
  (params (NewBody :type BP%20Body%20Object%20Reference))
  (if (!= NewBody self) ; Don't attach to self
    (bind _output_get (LocalVariables|SetOldCreation (Variables|Default|GetCreation)))
    (if (!= (Variables|BP_Body_C|GetCreation NewBody) _output_get) ; Belong to different creations?
      (bind _allparts (Default|GetAllMembers (LocalVariables|GetOldCreation)))
      (for _array_element _allparts
        (Variables|/Game/InventorySystem/Items/Parts/BP_Part.BP_Part_C|SetCreation _array_element (Variables|BP_Body_C|GetCreation NewBody))
        ;[1 1 1] Debug
        (Development|PrintString (Utilities|String|Append "Set Creation " (Utilities|GetDisplayName (Variables|BP_Body_C|GetCreation NewBody)) " for " (Utilities|GetDisplayName _array_element)) (Variables|Default|GetDEBUG_Print) true "(R=1.000000,G=0.186766,B=0.000000,A=1.000000)" 1e+02))
      (for _array_element_2 (Variables|/Game/InventorySystem/Items/Parts/BP_Creation.BP_Creation_C|GetBodies (LocalVariables|GetOldCreation))
        (if (and (Utilities|IsValid _array_element_2) (!= self _array_element_2))
          (Variables|BP_Body_C|SetCreation _array_element_2 (Variables|BP_Body_C|GetCreation NewBody))
          (Default|AddBody (Variables|BP_Body_C|GetCreation NewBody) _array_element_2)))
      (Actor|DestroyActor (LocalVariables|GetOldCreation))
      (else
        (for _array_element_3 (Variables|Default|GetMembers)
          (if (Utilities|Array|ContainsItem (Variables|BP_Body_C|GetMembers NewBody) _array_element_3)
            (return)))))
    ;[1 1 1] Debug
    (Development|PrintString (Utilities|String|Append "This body: " (Utilities|GetDisplayName self) " merged to new body " (Utilities|GetDisplayName NewBody)) (Variables|Default|GetDEBUG_Print) true "(R=1.000000,G=0.149158,B=0.000000,A=1.000000)" 1e+02)
    (for _array_element_4 (Variables|Default|GetMembers)
      (CallFunction|AddMember NewBody _array_element_4)
      (bind (_part _bodyindex _getbody _getpartcomponent _getattachcomp) (Default|GetREFs (CallFunction|AsPart _array_element_4) _array_element_4))
      (Default|SetBodyatIndex _part _bodyindex NewBody)
      (Transformation|AttachComponentToComponent _getattachcomp (Variables|BP_Body_C|GetBodyRoot NewBody) "None" "KeepWorld" "KeepWorld" "KeepWorld" true)
      ;[1 1 1] Debug
      (Development|PrintString (Utilities|String|Append (Utilities|GetDisplayName _getattachcomp) "   part attached to   " (Utilities|GetDisplayName (Variables|BP_Body_C|GetBodyRoot NewBody))) (Variables|Default|GetDEBUG_Print) true "(R=75.000000,G=75.000000,B=0.000000,A=1.000000)" 1e+02)
      (if (Utilities|DoesObjectImplementInterface _part "/Game/InventorySystem/Items/Parts/Joints/JointInterface.JointInterface_C")
        (Class|JointInterface|RepairJoint(Message) _part)))
    (Default|RemoveBody (Variables|BP_Body_C|GetCreation NewBody) self)
    (Actor|DestroyActor)))

(fn RemoveMember
  (params (Component :type Primitive%20Component%20Object%20Reference))
  (Utilities|IsValid Component
    (:Is%20Valid
      (Utilities|Array|RemoveItem (Variables|Default|GetMembers) Component)
      ;[1 1 1] Debug
      (Development|PrintString (Utilities|String|Append "Removing " (Utilities|GetDisplayName Component) " from body " (Utilities|GetObjectName self)) (Variables|Default|GetDEBUG_Print) true "(R=0.000000,G=0.660000,B=1.000000,A=1.000000)" 1e+02)
      (Variables|Default|SetNeedsRecalc true)
      (CallFunction|UpdateCOM))))

(fn AddMember
  (params (PartToAdd :type Primitive%20Component%20Object%20Reference))
  (Utilities|Array|AddUnique (Variables|Default|GetMembers) PartToAdd)
  (CallFunction|UpdateCOM))

(fn RecalcBody
  (bind _memberstocrawl (LocalVariables|GetMembersToCrawl))
  (bind _knownmembers (LocalVariables|GetKnownMembers))
  (bind _output (Utilities|Array|Get(acopy) _memberstocrawl))
  ;[1 1 1] While there are original members that need to be checked
  (Development|PrintString "Recalculating Bodies" (Variables|Default|GetDEBUG_Print) true "(R=0.000000,G=0.660000,B=1.000000,A=1.000000)" 1e+02)
  (Variables|Default|SetNeedsRecalc false)
  (LocalVariables|SetOriginalMembers (Variables|Default|GetMembers))
  (while (Utilities|IsValid (Utilities|Array|Get(acopy) (LocalVariables|GetOriginalMembers)))
    (Utilities|Array|Clear (LocalVariables|GetMembersToCrawl))
    (Utilities|Array|Clear (LocalVariables|GetKnownMembers))
    (Utilities|Array|Add (LocalVariables|GetMembersToCrawl) (Utilities|Array|Get(acopy) (LocalVariables|GetOriginalMembers)))
    ;[1 1 1] While there are members to crawl
    (while (Utilities|IsValid _output)
      (Development|PrintString (Utilities|String|Append "Crawling memeber: " (Utilities|GetDisplayName _output)) (Variables|Default|GetDEBUG_Print) true "(R=0.000000,G=0.660000,B=1.000000,A=1.000000)" 1e+02)
      (bind _output_get (LocalVariables|SetCurrentMember _output))
      (Utilities|Array|RemoveItem (LocalVariables|GetOriginalMembers) _output_get)
      (Utilities|Array|RemoveItem (LocalVariables|GetMembersToCrawl) (LocalVariables|GetCurrentMember))
      (Utilities|Array|AddUnique (LocalVariables|GetKnownMembers) (LocalVariables|GetCurrentMember))
      (bind _neighbors (Default|GetNeighbors (CallFunction|AsPart (LocalVariables|GetCurrentMember)) (LocalVariables|GetCurrentMember) true false))
      (for _array_element _neighbors
        (if (Utilities|Array|ContainsItem (LocalVariables|GetOriginalMembers) _array_element)
          (Utilities|Array|AddUnique (LocalVariables|GetMembersToCrawl) _array_element))))
    ;[1 1 1] Check if a new Body is needed
    (if (LocalVariables|GetCrawlingOriginalBody)
      (LocalVariables|SetCrawlingOriginalBody false)
      (Variables|Default|SetMembers (LocalVariables|GetKnownMembers))
      (CallFunction|CheckStillGrounded)
      (else
        (Development|PrintString "Need another body..." (Variables|Default|GetDEBUG_Print) true "(R=0.000000,G=0.660000,B=1.000000,A=1.000000)" 1e+02)
        (LocalVariables|SetGroundNewBody false)
        (bind _returnvalue (Game|SpawnActorfromClass "BP_Body_C" (Transformation|GetWorldTransform (Utilities|Array|Get(acopy) _knownmembers)) "AlwaysSpawn" 0 0 _knownmembers true 0))
        (bind _output_get_2 (LocalVariables|SetNewBody _returnvalue))
        (Utilities|Array|Add (LocalVariables|GetNewBodies) _output_get_2)
        (for _array_element_2 (LocalVariables|GetKnownMembers)
          (bind _output_get_3 (LocalVariables|SetCurrentMember _array_element_2))
          (if (Variables|/Game/InventorySystem/Items/Parts/BP_Part.BP_Part_C|GetIsGrounded (CallFunction|AsPart _output_get_3))
            (LocalVariables|SetGroundNewBody true))
          (Physics|SetSimulatePhysics (CallFunction|AsPrimitive (Variables|/Script/Engine.Actor|GetRootComponent (CallFunction|AsPart _output_get_3))) true)
          (Transformation|AttachComponentToComponent (Default|GetAttachComp (CallFunction|AsPart _output_get_3) _output_get_3) (Variables|BP_Body_C|GetBodyRoot (LocalVariables|GetNewBody)) "None" "KeepWorld" "KeepWorld" "KeepWorld" true)
          (Development|PrintString (Utilities|String|Append "Attaching " (Utilities|GetDisplayName (Default|GetAttachComp (CallFunction|AsPart _output_get_3) _output_get_3)) "  to body  " (Utilities|GetDisplayName (LocalVariables|GetNewBody))) (Variables|Default|GetDEBUG_Print) true "(R=0.000000,G=0.660000,B=1.000000,A=1.000000)" 1e+02)
          (Utilities|Array|SetArrayElem (Variables|/Game/InventorySystem/Items/Parts/BP_Part.BP_Part_C|GetBodies (CallFunction|AsPart (LocalVariables|GetCurrentMember))) (.BodyIndex (Default|GetBodyREF (CallFunction|AsPart (LocalVariables|GetCurrentMember)) (LocalVariables|GetCurrentMember))) (LocalVariables|GetNewBody))
          (if (Utilities|DoesObjectImplementInterface (CallFunction|AsPart (LocalVariables|GetCurrentMember)) "/Game/InventorySystem/Items/Parts/Joints/JointInterface.JointInterface_C")
            (Class|JointInterface|RepairJoint(Message) (CallFunction|AsPart (LocalVariables|GetCurrentMember)))))
        (Variables|BP_Body_C|SetDisableDestroy (LocalVariables|GetNewBody) false)
        (if (LocalVariables|GetGroundNewBody)
          (CallFunction|Ground (LocalVariables|GetNewBody))))))
  ;[1 1 1] Check if any Bodies need a new Creation
  (if (not (LocalVariables|GetCrawlingOriginalBody))
    (for _array_element_3 (LocalVariables|GetNewBodies)
      (bind _bodies (CallFunction|FindConnectedBodies _array_element_3))
      (bind _output_get_4 (LocalVariables|SetConnectedBodies _bodies))
      (if (Utilities|Array|ContainsItem _output_get_4 self)
        (Default|AddBody (Variables|Default|GetCreation) _array_element_3)
        (Development|PrintString (Utilities|String|Append (Utilities|GetDisplayName _array_element_3) " is still a body in original creation.") (Variables|Default|GetDEBUG_Print) true "(R=0.000000,G=0.660000,B=1.000000,A=1.000000)" 1e+02)
        (else
          (Development|PrintString (Utilities|String|Append (Utilities|GetDisplayName _array_element_3) " needs a new creation...") (Variables|Default|GetDEBUG_Print) true "(R=0.000000,G=0.660000,B=1.000000,A=1.000000)" 1e+02)
          (LocalVariables|SetNewCreation 0)
          (bind _array_element_4 (Utilities|Array|ForEachLoopwithBreak (LocalVariables|GetConnectedBodies) :!label _label)
            (:LoopBody
              (Utilities|IsValid (Variables|BP_Body_C|GetCreation _array_element_4)
                (:Is%20Valid
                  (if (!= (Variables|BP_Body_C|GetCreation _array_element_4) (Variables|Default|GetCreation))
                    (LocalVariables|SetNewCreation (Variables|BP_Body_C|GetCreation _array_element_4))
                    (goto _label Break)))))
            (:Completed
              (Utilities|IsValid (LocalVariables|GetNewCreation)
                (:Is%20Valid
                  _)
                (:Is%20Not%20Valid
                  (bind _returnvalue_2 (Game|SpawnActorfromClass "/Game/InventorySystem/Items/Parts/BP_Creation.BP_Creation_C" (Math|Transform|MakeTransform "0, 0, 0" "0, 0, 0" "1,1,1") "AlwaysSpawn" 0 true 0))
                  (LocalVariables|SetNewCreation _returnvalue_2)))
              (for _array_element_5 (LocalVariables|GetConnectedBodies)
                (Development|PrintString (Utilities|String|Append (Utilities|GetDisplayName _array_element_5) " moved to creation " (Utilities|GetDisplayName (LocalVariables|GetNewCreation))) (Variables|Default|GetDEBUG_Print) true "(R=0.000000,G=0.660000,B=1.000000,A=1.000000)" 1e+02)
                (Variables|BP_Body_C|SetCreation _array_element_5 (LocalVariables|GetNewCreation))
                (Default|AddBody (LocalVariables|GetNewCreation) _array_element_5)
                (for _array_element_6 (Variables|BP_Body_C|GetMembers _array_element_5)
                  (Variables|/Game/InventorySystem/Items/Parts/BP_Part.BP_Part_C|SetCreation (CallFunction|AsPart _array_element_6) (LocalVariables|GetNewCreation))))
              (Variables|/Game/InventorySystem/Items/Parts/BP_Creation.BP_Creation_C|SetDisableDestroy (LocalVariables|GetNewCreation) false))))))
    ;[1 1 1] Move WireNode references to correct Body
    (for _array_element_7 (Variables|Default|GetWireNodes)
      (Utilities|IsValid _array_element_7
        (:Is%20Valid
          (bind _output_get_5 (LocalVariables|SetCurrentWireNode _array_element_7))
          (Utilities|IsValid (Variables|/Game/InventorySystem/Wires/BP_WireNode.BP_WireNode_C|GetComponentPlacedOn _output_get_5)
            (:Is%20Valid
              (if (not (Utilities|Array|ContainsItem (Variables|Default|GetMembers) (Variables|/Game/InventorySystem/Wires/BP_WireNode.BP_WireNode_C|GetComponentPlacedOn _output_get_5)))
                (Utilities|Array|RemoveItem (Variables|Default|GetWireNodes) _output_get_5)
                (Utilities|Array|Add (Variables|BP_Body_C|GetWireNodes (.GetBody (Default|GetBodyREF (CallFunction|AsPart (Variables|/Game/InventorySystem/Wires/BP_WireNode.BP_WireNode_C|GetComponentPlacedOn _output_get_5)) (Variables|/Game/InventorySystem/Wires/BP_WireNode.BP_WireNode_C|GetComponentPlacedOn _output_get_5)))) _output_get_5)
                (Default|DrawWires _output_get_5)))))))))

(fn EndStasis
  (bind _bodyroot (Variables|Default|GetBodyRoot))
  (Physics|SetEnableGravity _bodyroot true)
  (Class|PrimitiveComponent|SetAngularDamping _bodyroot 0.0)
  (for _array_element (Variables|Default|GetMembers)
    (if (Utilities|DoesObjectImplementInterface (CallFunction|AsPart _array_element) "/Game/InventorySystem/Items/Parts/Joints/JointInterface.JointInterface_C")
      (Class|JointInterface|UnlockJoint(Message) (CallFunction|AsPart _array_element)))))

(fn BeginStasis
  (bind _bodyroot (Variables|Default|GetBodyRoot))
  (Physics|SetEnableGravity _bodyroot false)
  (Class|PrimitiveComponent|SetAngularDamping _bodyroot (Variables|Default|GetStasisDamping))
  (for _array_element (Variables|Default|GetMembers)
    (if (Utilities|DoesObjectImplementInterface (CallFunction|AsPart _array_element) "/Game/InventorySystem/Items/Parts/Joints/JointInterface.JointInterface_C")
      (Class|JointInterface|LockJoint(Message) (CallFunction|AsPart _array_element)))))

(fn Ground
  (Variables|Default|SetIsGrounded true)
  (Physics|SetSimulatePhysics (Variables|Default|GetBodyRoot) false)
  (for _array_element (Variables|Default|GetMembers)
    (if (Utilities|DoesObjectImplementInterface (CallFunction|AsPart _array_element) "/Game/InventorySystem/Items/Parts/Joints/JointInterface.JointInterface_C")
      (Class|JointInterface|RepairJoint(Message) (CallFunction|AsPart _array_element)))))

(fn Unground
  (if (Variables|Default|GetIsGrounded)
    (Physics|SetSimulatePhysics (Variables|Default|GetBodyRoot) true)
    (Variables|Default|SetIsGrounded false)
    (for _array_element (Variables|Default|GetMembers)
      (Variables|/Game/InventorySystem/Items/Parts/BP_Part.BP_Part_C|SetIsGrounded (CallFunction|AsPart _array_element) false))))

(fn RepairJoints
  (for _array_element (Variables|Default|GetMembers)
    (if (Utilities|DoesObjectImplementInterface (CallFunction|AsPart _array_element) "/Game/InventorySystem/Items/Parts/Joints/JointInterface.JointInterface_C")
      (Class|JointInterface|RepairJoint(Message) (CallFunction|AsPart _array_element)))))

(fn UpdateCOM
  (bind _bodyroot (Variables|Default|GetBodyRoot))
  (for _array_element (Variables|Default|GetMembers)
    (Utilities|IsValid _array_element
      (:Is%20Valid
        (LocalVariables|SetSumCOM (+ (LocalVariables|GetSumCOM) (Physics|GetCenterOfMass _array_element "None")))
        (Math|Integer|IncrementInt (LocalVariables|GetPartCount)))))
  (Class|PrimitiveComponent|SetCenterOfMass _bodyroot (- (/ (LocalVariables|GetSumCOM) (LocalVariables|GetPartCount)) (Transformation|GetWorldLocation _bodyroot)) "None"))

(fn AddWireNode
  (params (WireNode :type BP%20Wire%20Node%20Object%20Reference))
  (Utilities|Array|AddUnique (Variables|Default|GetWireNodes) WireNode))

(fn RemoveWireNode
  (params (WireNode :type BP%20Wire%20Node%20Object%20Reference))
  (Utilities|Array|RemoveItem (Variables|Default|GetWireNodes) WireNode))

(fn FindConnectedBodies
  (bind _bodiestocrawl (LocalVariables|GetBodiesToCrawl))
  (bind _output (Utilities|Array|Get(acopy) _bodiestocrawl))
  (Utilities|Array|Add _bodiestocrawl self)
  (while (Utilities|IsValid _output)
    (bind _output_get (LocalVariables|SetCurrentBody _output))
    (Utilities|Array|AddUnique (LocalVariables|GetKnownBodies) _output_get)
    (Utilities|Array|RemoveIndex (LocalVariables|GetBodiesToCrawl))
    (for _array_element (Variables|BP_Body_C|GetMembers (LocalVariables|GetCurrentBody))
      (if (Utilities|DoesObjectImplementInterface (CallFunction|AsPart _array_element) "/Game/InventorySystem/Items/Parts/Joints/JointInterface.JointInterface_C")
        (for _array_element_2 (Variables|/Game/InventorySystem/Items/Parts/BP_Part.BP_Part_C|GetBodies (CallFunction|AsPart _array_element))
          (if (not (Utilities|Array|ContainsItem (LocalVariables|GetKnownBodies) _array_element_2))
            (Utilities|Array|AddUnique (LocalVariables|GetBodiesToCrawl) _array_element_2))))))
  (return (LocalVariables|GetKnownBodies)))

(fn CheckStillGrounded
  (if (not (Physics|IsSimulatingPhysics (Variables|Default|GetBodyRoot) "None"))
    (for _array_element (Variables|Default|GetMembers)
      (if (Variables|/Game/InventorySystem/Items/Parts/BP_Part.BP_Part_C|GetIsGrounded (CallFunction|AsPart _array_element))
        (return)))
    (Physics|SetSimulatePhysics (Variables|Default|GetBodyRoot) true)
    (Variables|Default|SetIsGrounded false)))

(fn DeleteBody
  (for _array_element (Variables|Default|GetWireNodes)
    (Actor|DestroyActor _array_element))
  (for _array_element_2 (Variables|Default|GetMembers)
    (Utilities|IsValid _array_element_2
      (:Is%20Valid
        (Actor|DestroyActor (CallFunction|AsPart _array_element_2)))))
  (Actor|DestroyActor))

(fn RedrawAllWires
  (for _array_element (Variables|Default|GetWireNodes)
    (Default|DrawWires _array_element)))