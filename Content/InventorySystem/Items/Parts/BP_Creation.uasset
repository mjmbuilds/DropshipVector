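; BP_Creation is the manager actor for a built creation, tracking its Bodies, each holding member Parts and wire nodes.
; It forwards stasis, physics, unground, teleport, wire redraw and delete operations to its Bodies, and destroys itself when none remain unless disabled.
; Shattering detaches parts with random impulses before destroying Bodies.
; The antigrav variant floats red-tinted parts with damping, removes wires, then restores gravity after a short delay.
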(event Custom|ShatterCreationAntigravDelay
  (Utilities|FlowControl|Delay 0.5)
  (for _array_element (Variables|Default|GetTempPartsForDestroy)
    (Utilities|IsValid _array_element
      (:Is%20Valid
        (Physics|SetEnableGravity (CallFunction|AsPrimitive (Variables|/Script/Engine.Actor|GetRootComponent _array_element)) true)
        (Class|PrimitiveComponent|SetLinearDamping (CallFunction|AsPrimitive (Variables|/Script/Engine.Actor|GetRootComponent _array_element)) 0.0))))
  (Actor|DestroyActor))

(event EventBeginPlay
  ;[1 1 1] Debug
  (Development|PrintString (Utilities|String|Append (Utilities|GetDisplayName self) " Created") true true "(R=0.500000,G=0.000000,B=1.000000,A=1.000000)" 1e+02))

(event EventEndPlay
  (params (EndPlayReason :type EEndPlayReason%20Enum :default "Destroyed"))
  ;[1 1 1] Debug
  (Development|PrintString (Utilities|String|Append (Utilities|GetDisplayName self) " was Destroyed") true true "(R=0.250000,G=0.000000,B=0.500000,A=1.000000)" 1e+02))

(event EventTick
  (params (DeltaSeconds :type Float%20%28single-precision%29))
  (if (< (Utilities|Array|Length (Variables|Default|GetBodies)) 1)
    (if (not (Variables|Default|GetDisableDestroy))
      (Actor|DestroyActor))))

(fn ConstructionScript)

(fn AddBody
  (params (BodyToAdd :type BP%20Body%20Object%20Reference))
  (Utilities|Array|AddUnique (Variables|Default|GetBodies) BodyToAdd))

(fn RemoveBody
  (params (BodyToRemove :type BP%20Body%20Object%20Reference))
  (Utilities|Array|RemoveItem (Variables|Default|GetBodies) BodyToRemove))

(fn GetAllMembers
  (for _array_element (Variables|Default|GetBodies)
    (Utilities|IsValid _array_element
      (:Is%20Valid
        (for _array_element_2 (Variables|/Game/InventorySystem/Items/Parts/BP_Body.BP_Body_C|GetMembers _array_element)
          (Utilities|Array|AddUnique (LocalVariables|GetReturnParts) (CallFunction|AsPart _array_element_2))))))
  (return (LocalVariables|GetReturnParts)))

(fn ShatterCreation
  (params (DestroyParts :type Boolean))
  (bind _allparts (CallFunction|GetAllMembers))
  (for _array_element _allparts
    (Variables|/Game/InventorySystem/Items/Parts/BP_Part.BP_Part_C|SetCreation _array_element 0)
    (Variables|/Game/InventorySystem/Items/Parts/BP_Part.BP_Part_C|SetBodies _array_element (LocalVariables|GetEmptyBodies))
    (Transformation|DetachFromComponent (Variables|/Script/Engine.Actor|GetRootComponent _array_element) "KeepWorld" "KeepWorld" "KeepWorld" true)
    (Physics|SetSimulatePhysics (CallFunction|AsPrimitive (Variables|/Script/Engine.Actor|GetRootComponent _array_element)) true)
    (Physics|AddImpulseatLocation (CallFunction|AsPrimitive (Variables|/Script/Engine.Actor|GetRootComponent _array_element)) (* (Math|Random|RandomUnitVector) (LocalVariables|GetShatterForce)) (Transformation|GetActorLocation _array_element) "None")
    (if DestroyParts
      (Variables|/Game/InventorySystem/Items/Parts/BP_Part.BP_Part_C|SetDestroyTimer _array_element (+ (Math|Random|RandomInteger 150) 50))))
  (bind _output_get (LocalVariables|SetTempBodies (Variables|Default|GetBodies)))
  (for _array_element_2 _output_get
    (Utilities|IsValid _array_element_2
      (:Is%20Valid
        (Actor|DestroyActor _array_element_2))))
  (Actor|DestroyActor))

(fn EndStasis
  (Variables|Default|SetInStasis false)
  (for _array_element (Variables|Default|GetBodies)
    (Default|EndStasis _array_element)))

(fn BeginStasis
  (Variables|Default|SetInStasis true)
  (for _array_element (Variables|Default|GetBodies)
    (Default|BeginStasis _array_element)))

(fn UngroundCreation
  (for _array_element (Variables|Default|GetBodies)
    (Default|Unground _array_element)))

(fn EnablePhysics
  (for _array_element (Variables|Default|GetBodies)
    (Physics|SetSimulatePhysics (Variables|/Game/InventorySystem/Items/Parts/BP_Body.BP_Body_C|GetBodyRoot _array_element) true)))

(fn DisablePhysics
  (for _array_element (Variables|Default|GetBodies)
    (Physics|SetSimulatePhysics (Variables|/Game/InventorySystem/Items/Parts/BP_Body.BP_Body_C|GetBodyRoot _array_element) false)))

(fn TeleportOffset
  (params (OffsetVector :type Vector))
  (for _array_element (Variables|Default|GetBodies)
    (Utilities|IsValid _array_element
      (:Is%20Valid
        (Transformation|SetWorldLocation (Variables|/Script/Engine.Actor|GetRootComponent _array_element) (+ (Transformation|GetActorLocation _array_element) OffsetVector) false true)))))

(fn GetAllWires
  (bind _allwirenodes (LocalVariables|GetAllWireNodes))
  (for _array_element (Variables|Default|GetBodies)
    (Utilities|IsValid _array_element
      (:Is%20Valid
        (for _array_element_2 (Variables|/Game/InventorySystem/Items/Parts/BP_Body.BP_Body_C|GetWireNodes _array_element)
          (Utilities|IsValid _array_element_2
            (:Is%20Valid
              (Utilities|Array|Add _allwirenodes _array_element_2)
              (return _allwirenodes))))))))

(fn DeleteCreation
  (for _array_element (Variables|Default|GetBodies)
    (Default|DeleteBody _array_element))
  (Actor|DestroyActor))

(fn RedrawAllWires
  (for _array_element (Variables|Default|GetBodies)
    (Default|RedrawAllWires _array_element)))

(fn ShatterCreationAntigrav
  (bind _allparts (CallFunction|GetAllMembers))
  (bind _output_get (LocalVariables|SetTempMembers _allparts))
  (for _array_element _output_get
    (Transformation|DetachFromComponent (Variables|/Script/Engine.Actor|GetRootComponent _array_element) "KeepWorld" "KeepWorld" "KeepWorld" true)
    (Physics|SetSimulatePhysics (CallFunction|AsPrimitive (Variables|/Script/Engine.Actor|GetRootComponent _array_element)) true)
    (Physics|SetEnableGravity (CallFunction|AsPrimitive (Variables|/Script/Engine.Actor|GetRootComponent _array_element)) false)
    (Class|PrimitiveComponent|SetLinearDamping (CallFunction|AsPrimitive (Variables|/Script/Engine.Actor|GetRootComponent _array_element)) 1e+01)
    (Physics|AddImpulseatLocation (CallFunction|AsPrimitive (Variables|/Script/Engine.Actor|GetRootComponent _array_element)) (* (+ (Math|Random|RandomUnitVector) "0, 0,1.000000") 5e+04) (Transformation|GetActorLocation _array_element) "None")
    (Variables|/Game/InventorySystem/Items/Parts/BP_Part.BP_Part_C|SetDestroyTimer _array_element (+ (Math|Random|RandomInteger 150) 150))
    (for _array_element_2 (Actor|GetComponentsByClass _array_element "/Script/Engine.PrimitiveComponent")
      (for _index (range 0 (- (Rendering|Material|GetNumMaterials _array_element_2) 1))
        (Rendering|Material|SetMaterial _array_element_2 _index "/Game/Materials/M_ProjectileRed.M_ProjectileRed")))
    (bind _wires (CallFunction|GetAllWires))
    (for _array_element_3 _wires
      (Utilities|IsValid _array_element_3
        (:Is%20Valid
          (Actor|DestroyActor _array_element_3)))))
  (CallFunction|ShatterCreationAntigravDelay)
  (Variables|Default|SetTempPartsForDestroy (LocalVariables|GetTempMembers))
  (bind _output_get_2 (LocalVariables|SetTempBodies (Variables|Default|GetBodies)))
  (for _array_element_4 _output_get_2
    (Utilities|IsValid _array_element_4
      (:Is%20Valid
        (Actor|DestroyActor _array_element_4)))))