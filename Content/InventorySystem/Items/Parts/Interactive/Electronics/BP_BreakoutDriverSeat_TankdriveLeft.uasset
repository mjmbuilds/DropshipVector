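; Electronics breakout part that converts a connected driver seat's controls into a left-side tank drive power signal.
; Each tick, unless DestroyTimer is running, it follows its first input wire to the parent BP_DriverSeat.
; Power is the seat's throttled power plus steering multiplied by gear.
; Non-zero power marks the part Active and brightens the logic box display glow; zero dims it and clears Active.
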(event EventTick
  (params (DeltaSeconds :type Float%20%28single-precision%29))
  (bind _logicboxdisplay (Variables|Default|GetLogicBoxDisplay))
  (bind _inputwires (Variables|Default|GetInputWires))
  (bind _output (Utilities|Array|Get(acopy) _inputwires))
  (|CallParentFunction DeltaSeconds)
  (if (< (Variables|Default|GetDestroyTimer) 0)
    (if (CallFunction|HasAnyInputWire)
      (Utilities|IsValid _output
        (:Is%20Valid
          (bind (_hasconnection _parentconnection) (Default|GetParentConnection _output))
          (if _hasconnection
            (bind _asbp_driver_seat (Utilities|Casting|CastToBP_DriverSeat _parentconnection))
            (bind _output_get (Variables|Default|SettempPower (Variables|/Game/InventorySystem/Items/Parts/Interactive/Seats/BP_DriverSeat.BP_DriverSeat_C|GetThrottledPower _asbp_driver_seat)))
            (bind _output_get_2 (Variables|Default|SetPower (+ _output_get (* (Variables|/Game/InventorySystem/Items/Parts/Interactive/Seats/BP_DriverSeat.BP_DriverSeat_C|GetSteering _asbp_driver_seat) (Variables|/Game/InventorySystem/Items/Parts/Interactive/Seats/BP_DriverSeat.BP_DriverSeat_C|GetGear _asbp_driver_seat)))))
            (if (!= _output_get_2 0.0)
              (Rendering|Material|SetScalarParameterValueonMaterials _logicboxdisplay "Glow" 6.0)
              (Variables|Default|SetActive true)
              (else
                (Rendering|Material|SetScalarParameterValueonMaterials _logicboxdisplay "Glow" 0.5)
                (Variables|Default|SetActive false)))))))))

(fn ConstructionScript
  (|CallParentFunction))