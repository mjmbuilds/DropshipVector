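; BP_PartInteractive is an interactive part in the inventory item system that tracks the parents wired into it.
; It holds them in an InputWires array, adding a parent uniquely only while the count is below MaxParents.
; Helper functions remove a parent, check for free capacity and report whether any input wire exists.
; It has no active event logic, and its construction script only calls the parent version.
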(event EventBeginPlay
  (|CallParentFunction) ; This node is disabled and will not be called.\nDrag off pins to build functionality.
)

(event Collision|EventActorBeginOverlap
  (params (OtherActor :type Actor%20Object%20Reference)))

(event EventTick
  (params (DeltaSeconds :type Float%20%28single-precision%29))
  (|CallParentFunction DeltaSeconds) ; This node is disabled and will not be called.\nDrag off pins to build functionality.
)

(fn ConstructionScript
  (|CallParentFunction))

(fn HasAnyInputWire
  (return (> (Utilities|Array|Length (Variables|Default|GetInputWires)) 0)))

(fn AddInputWire
  (params (ParentToAdd :type BP%20Wire%20Node%20Object%20Reference))
  (if (CallFunction|CanAcceptParent)
    (Utilities|Array|AddUnique (Variables|Default|GetInputWires) ParentToAdd)))

(fn RemoveParent
  (params (ParentToRemove :type BP%20Wire%20Node%20Object%20Reference))
  (Utilities|Array|RemoveItem (Variables|Default|GetInputWires) ParentToRemove))

(fn CanAcceptParent
  (return (< (Utilities|Array|Length (Variables|Default|GetInputWires)) (Variables|Default|GetMaxParents))))