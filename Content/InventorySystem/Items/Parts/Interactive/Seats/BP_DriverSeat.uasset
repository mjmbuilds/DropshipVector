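; Driver seat part that a FirstPersonCharacter enters or leaves by interacting, holding driving input state.
; TrySeat attaches the player with collision disabled and a switched camera probe channel, then on exit detaches them above the seat and clears inputs.
; While occupied, Tick ramps Steering from the A/D flags, self-centering otherwise, and clears one-shot shift flags.
; ShiftUp and ShiftDown step Gear, which scales Power into ThrottledPower.
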(event EventBeginPlay
  (|CallParentFunction) ; This node is disabled and will not be called.\nDrag off pins to build functionality.
)

(event EventInteractClick
  (params (Interactor :type Actor%20Object%20Reference))
  (bind _asfirst_person_character (Utilities|Casting|CastToFirstPersonCharacter Interactor))
  (CallFunction|TrySeat _asfirst_person_character))

(event EventTick
  (params (DeltaSeconds :type Float%20%28single-precision%29))
  (|CallParentFunction DeltaSeconds)
  (Utilities|IsValid (Variables|Default|GetPlayerInSeat)
    (:Is%20Valid
      (if (Variables|Default|GetThrottleUp)
        (Variables|Default|SetThrottleUp false))
      (if (Variables|Default|GetThrottleDown)
        (Variables|Default|SetThrottleDown false))
      (if (Variables|Default|GetA_Active)
        (CallFunction|SteerLeft)
        (elif (Variables|Default|GetD_Active)
          (CallFunction|SteerRight)
          (else
            (CallFunction|SteerCenter)))))))

(fn ConstructionScript
  (|CallParentFunction))

(fn PlayerExitSeat
  (Variables|Default|SetActive false)
  (Variables|Default|SetPower 0.0)
  (Variables|Default|SetThrottledPower 0.0)
  (Variables|Default|SetSteering 0.0)
  (Variables|Default|SetW_Active false)
  (Variables|Default|SetS_Active false)
  (Variables|Default|SetA_Active false)
  (Variables|Default|SetD_Active false)
  (Variables|Default|SetPlayerInSeat 0))

(fn SteerLeft
  (if (> (Variables|Default|GetSteering) -1.0)
    (Variables|Default|SetSteering (Math|Float|Clamp(Float) (- (Variables|Default|GetSteering) (Variables|Default|GetSteerSpeed)) -1.0))))

(fn SteerRight
  (if (< (Variables|Default|GetSteering) 1.0)
    (Variables|Default|SetSteering (Math|Float|Clamp(Float) (+ (Variables|Default|GetSteering) (Variables|Default|GetSteerSpeed)) -1.0))))

(fn SteerCenter
  (if (> (Variables|Default|GetSteering) 0.0)
    (Variables|Default|SetSteering (Math|Float|Clamp(Float) (- (Variables|Default|GetSteering) (Variables|Default|GetSteerSpeed))))
    (elif (< (Variables|Default|GetSteering) 0.0)
      (Variables|Default|SetSteering (Math|Float|Clamp(Float) (+ (Variables|Default|GetSteering) (Variables|Default|GetSteerSpeed)) -1.0 0.0)))))

(fn ShiftUp
  (Variables|Default|SetThrottleUp true)
  (Variables|Default|SetGear (Math|Float|Clamp(Float) (+ (Variables|Default|GetGear) 0.1)))
  (CallFunction|SetThrottledPower))

(fn ShiftDown
  (Variables|Default|SetThrottleDown true)
  (Variables|Default|SetGear (Math|Float|Clamp(Float) (+ (Variables|Default|GetGear) -0.1)))
  (CallFunction|SetThrottledPower))

(fn SetThrottledPower
  (Variables|Default|SetThrottledPower (* (Variables|Default|GetPower) (Variables|Default|GetGear))))

(fn AdjustSteerSpeed
  (params (SteerSpeed :type Float%20%28single-precision%29))
  (Variables|Default|SetSteerSpeed SteerSpeed))

(fn TrySeat
  (params (Player :type First%20Person%20Character%20Object%20Reference))
  (bind _self self)
  (bind _rootcomponent (Variables|/Script/Engine.Actor|GetRootComponent _self))
  (bind _returnvalue (Transformation|GetWorldTransform _rootcomponent))
  (bind (_location _rotation) (Math|Transform|BreakTransform _returnvalue))
  (Utilities|IsValid (Variables|Default|GetPlayerInSeat)
    (:Is%20Valid
      (if (== (Variables|Default|GetPlayerInSeat) Player)
        (Variables|/Game/PlayerCharacter/FirstPersonCharacter.FirstPersonCharacter_C|SetSeat Player 0)
        (Transformation|DetachFromComponent (Variables|/Script/Engine.Character|GetCapsuleComponent (Variables|Default|GetPlayerInSeat)) "KeepWorld" "KeepWorld" "KeepWorld" true)
        (Collision|SetCollisionProfileName (Variables|/Script/Engine.Character|GetCapsuleComponent (Variables|Default|GetPlayerInSeat)) "Pawn" :!class /Script/Engine.PrimitiveComponent)
        (Collision|SetCollisionProfileName (Variables|/Script/Engine.Character|GetMesh (Variables|Default|GetPlayerInSeat)) "CharacterMesh" :!class /Script/Engine.PrimitiveComponent)
        (Collision|SetCollisionProfileName (Variables|/Game/PlayerCharacter/FirstPersonCharacter.FirstPersonCharacter_C|GetMesh2P (Variables|Default|GetPlayerInSeat)) "CharacterMesh" :!class /Script/Engine.PrimitiveComponent)
        (Transformation|SetWorldLocationAndRotation (Variables|/Script/Engine.Character|GetCapsuleComponent (Variables|Default|GetPlayerInSeat)) (Math|Vector|MakeVector (.x (Transformation|GetWorldLocation (Variables|/Script/Engine.Character|GetCapsuleComponent (Variables|Default|GetPlayerInSeat)))) (.y (Transformation|GetWorldLocation (Variables|/Script/Engine.Character|GetCapsuleComponent (Variables|Default|GetPlayerInSeat)))) (+ (.z (Transformation|GetWorldLocation (Variables|/Script/Engine.Character|GetCapsuleComponent (Variables|Default|GetPlayerInSeat)))) 2e+02)) (Math|Rotator|MakeRotator 0.0 0.0 (.yaw (Transformation|GetWorldRotation (Variables|/Script/Engine.Character|GetCapsuleComponent (Variables|Default|GetPlayerInSeat))))) false true)
        (Variables|/Script/Engine.SpringArmComponent|SetProbeChannel (Variables|/Game/PlayerCharacter/FirstPersonCharacter.FirstPersonCharacter_C|GetCameraBoom (Variables|Default|GetPlayerInSeat)) "ECC_Camera")
        (CallFunction|PlayerExitSeat)))
    (:Is%20Not%20Valid
      (Variables|Default|SetActive true)
      (Variables|Default|SetPlayerInSeat Player)
      (Variables|/Game/PlayerCharacter/FirstPersonCharacter.FirstPersonCharacter_C|SetSeat Player self)
      (Collision|SetCollisionProfileName (Variables|/Script/Engine.Character|GetCapsuleComponent (Variables|Default|GetPlayerInSeat)) "NoCollision" :!class /Script/Engine.PrimitiveComponent)
      (Collision|SetCollisionProfileName (Variables|/Script/Engine.Character|GetMesh (Variables|Default|GetPlayerInSeat)) "NoCollision" :!class /Script/Engine.PrimitiveComponent)
      (Collision|SetCollisionProfileName (Variables|/Game/PlayerCharacter/FirstPersonCharacter.FirstPersonCharacter_C|GetMesh2P (Variables|Default|GetPlayerInSeat)) "NoCollision" :!class /Script/Engine.PrimitiveComponent)
      (Transformation|SetWorldLocationAndRotation (Variables|/Script/Engine.Actor|GetRootComponent (Variables|Default|GetPlayerInSeat)) (+ (+ (* (Math|Vector|GetUpVector _rootcomponent) 5.0) (* (Math|Vector|GetForwardVector _rootcomponent) -3e+01)) _location) _rotation false false)
      (Transformation|AttachComponentToComponent (Variables|/Script/Engine.Character|GetCapsuleComponent (Variables|Default|GetPlayerInSeat)) (Variables|/Script/Engine.Actor|GetRootComponent self) "None" "KeepWorld" "KeepWorld" "KeepWorld" true)
      (Variables|/Script/Engine.SpringArmComponent|SetProbeChannel (Variables|/Game/PlayerCharacter/FirstPersonCharacter.FirstPersonCharacter_C|GetCameraBoom (Variables|Default|GetPlayerInSeat)) "ECC_GameTraceChannel12"))))