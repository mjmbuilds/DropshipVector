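; Motor part for player creations that spins a physics constraint between its two bodies according to the power on its first input wire.
; Each tick, unless destroyed or in stasis, it scales wire power by engine speed into an angular velocity target, driven at engine strength.
; It toggles twist orientation drive when stopping or moving.
; Joint events lock or free the twist axis and reconnect the bodies for repair.
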(event EventTick
  (params (DeltaSeconds :type Float%20%28single-precision%29))
  (bind _engineconstraint (Variables|Default|GetEngineConstraint))
  (|CallParentFunction DeltaSeconds)
  (if (< (Variables|Default|GetDestroyTimer) 0)
    (if (CallFunction|HasAnyInputWire)
      (bind (_hasconnection _parentconnection) (Default|GetParentConnection (Utilities|Array|Get(acopy) (Variables|Default|GetInputWires))))
      (if _hasconnection
        (if (not (Variables|/Game/InventorySystem/Items/Parts/BP_Creation.BP_Creation_C|GetInStasis (Variables|Default|GetCreation)))
          (Class|PhysicsConstraintComponent|SetAngularVelocityTarget _engineconstraint (Math|Vector|MakeVector (* (Variables|/Game/InventorySystem/Items/Parts/Interactive/BP_PartInteractive.BP_PartInteractive_C|GetPower _parentconnection) (Variables|Default|GetEngineSpeed)) 0.0 0.0))
          (Class|PhysicsConstraintComponent|SetAngularDriveParams _engineconstraint 0.0 (Variables|Default|GetEngineStrength) 0.0)
          (if (== (* (Variables|/Game/InventorySystem/Items/Parts/Interactive/BP_PartInteractive.BP_PartInteractive_C|GetPower _parentconnection) (Variables|Default|GetEngineSpeed)) 0.0)
            (if (Variables|Default|GetTempWasMoving)
              (Variables|Default|SetTempWasMoving false)
              (Class|PhysicsConstraintComponent|SetOrientationDriveTwistandSwing _engineconstraint true false)
              (Class|PhysicsConstraintComponent|SetAngularOrientationTarget _engineconstraint (Math|Rotator|MakeRotator (.roll (Variables|/Script/Engine.SceneComponent|GetRelativeRotation _engineconstraint)) 0.0 0.0)))
            (else
              (Variables|Default|SetTempWasMoving true)
              (Class|PhysicsConstraintComponent|SetOrientationDriveTwistandSwing _engineconstraint false false))))))))

(event EventUnlockJoint
  (Class|PhysicsConstraintComponent|SetAngularTwistLimit (Variables|Default|GetEngineConstraint) "ACM_Free" 0.0))

(event EventLockJoint
  (Class|PhysicsConstraintComponent|SetAngularTwistLimit (Variables|Default|GetEngineConstraint) "ACM_Locked" 0.0)
  (Class|PrimitiveComponent|WakeAllRigidBodies (CallFunction|AsPrimitive (Variables|Transformation|GetRootComponent self))))

(event EventRepairJoint
  (Class|PhysicsConstraintComponent|SetConstrainedComponents (Variables|Default|GetEngineConstraint) (Variables|/Game/InventorySystem/Items/Parts/BP_Body.BP_Body_C|GetBodyRoot (Utilities|Array|Get(acopy) (Variables|Default|GetBodies) 1)) "None" (Variables|/Game/InventorySystem/Items/Parts/BP_Body.BP_Body_C|GetBodyRoot (Utilities|Array|Get(acopy) (Variables|Default|GetBodies))) "None"))

(fn ConstructionScript
  (|CallParentFunction))