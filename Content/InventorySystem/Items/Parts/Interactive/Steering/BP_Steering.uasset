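; BP_Steering is an interactive steering part for player creations that turns a servo joint between its two bodies.
; Each tick, outside stasis and before destruction, it scales the first input wire's power by SteerAngle into the roll target of the angular drive on ServoConstraint.
; Joint events free or lock the constraint's twist axis, waking bodies on lock, or re-bind both bodies for repair.
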(event EventTick
  (params (DeltaSeconds :type Float%20%28single-precision%29))
  (bind _servoconstraint (Variables|Default|GetServoConstraint))
  (|CallParentFunction DeltaSeconds)
  (if (< (Variables|Default|GetDestroyTimer) 0)
    (if (CallFunction|HasAnyInputWire)
      (bind (_hasconnection _parentconnection) (Default|GetParentConnection (Utilities|Array|Get(acopy) (Variables|Default|GetInputWires))))
      (if _hasconnection
        (if (not (Variables|/Game/InventorySystem/Items/Parts/BP_Creation.BP_Creation_C|GetInStasis (Variables|Default|GetCreation)))
          (Class|PhysicsConstraintComponent|SetAngularOrientationTarget _servoconstraint (Math|Rotator|MakeRotator (* (Variables|/Game/InventorySystem/Items/Parts/Interactive/BP_PartInteractive.BP_PartInteractive_C|GetPower _parentconnection) (Variables|Default|GetSteerAngle)) 0.0 0.0))
          (Class|PhysicsConstraintComponent|SetAngularDriveParams _servoconstraint (Variables|Default|GetTEMP_Strength) 0.0 0.0))))))

(event EventRepairJoint
  (Class|PhysicsConstraintComponent|SetConstrainedComponents (Variables|Default|GetServoConstraint) (Variables|/Game/InventorySystem/Items/Parts/BP_Body.BP_Body_C|GetBodyRoot (Utilities|Array|Get(acopy) (Variables|Default|GetBodies) 1)) "None" (Variables|/Game/InventorySystem/Items/Parts/BP_Body.BP_Body_C|GetBodyRoot (Utilities|Array|Get(acopy) (Variables|Default|GetBodies))) "None"))

(event EventLockJoint
  (Class|PhysicsConstraintComponent|SetAngularTwistLimit (Variables|Default|GetServoConstraint) "ACM_Locked" 0.0)
  (Class|PrimitiveComponent|WakeAllRigidBodies (CallFunction|CompasPrimitive (Variables|Transformation|GetRootComponent self))))

(event EventUnlockJoint
  (Class|PhysicsConstraintComponent|SetAngularTwistLimit (Variables|Default|GetServoConstraint) "ACM_Free" 0.0))

(fn ConstructionScript
  (|CallParentFunction))