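; Wire node placed on part components, linking interactive parts through branching chains with one previous and many next nodes.
; Head and tail nodes are color-coded; tails register as inputs on their interactive part, and parent lookups recurse back to the head, setting glow by its active state.
; DrawWires spawns a BP_Wire per link, marking cross-body wires dynamic and attaching the rest.
; Nodes unlink and destroy themselves when their component becomes invalid.
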(event EventTick
  (params (DeltaSeconds :type Float%20%28single-precision%29))
  (Utilities|IsValid (Variables|Default|GetComponentPlacedOn)
    (:Is%20Not%20Valid
      (CallFunction|RemoveWireNode))))

(event EventBeginPlay
  (Rendering|Material|SetVectorParameterValueonMaterials (Variables|Default|GetWireNodeRoot) "Color" (Variables|Default|GetDefaultColor)))

(fn ConstructionScript
  (|CallParentFunction))

(fn DrawWires
  (bind _wires (Variables|Default|GetWires))
  (bind _componentplacedon (Variables|Default|GetComponentPlacedOn))
  (for _array_element _wires
    (Utilities|IsValid _array_element
      (:Is%20Valid
        (Actor|DestroyActor _array_element))))
  (Utilities|Array|Clear _wires)
  (for _array_element_2 (Variables|Default|GetNextWireNodes)
    (Utilities|IsValid _array_element_2
      (:Is%20Valid
        (bind _returnvalue (Game|SpawnActorfromClass "/Game/InventorySystem/Wires/BP_Wire.BP_Wire_C" (Transformation|GetActorTransform) "AlwaysSpawn" 0 self _array_element_2 (!= (.GetBody (Default|GetBodyREF (CallFunction|AsPart (Variables|BP_WireNode_C|GetComponentPlacedOn _array_element_2)) (Variables|BP_WireNode_C|GetComponentPlacedOn _array_element_2))) (.GetBody (Default|GetBodyREF (CallFunction|AsPart _componentplacedon) _componentplacedon))) 0))
        (Utilities|Array|Add (Variables|Default|GetWires) _returnvalue)
        (if (not (Variables|/Game/InventorySystem/Wires/BP_Wire.BP_Wire_C|GetIsDynamic _returnvalue))
          (Transformation|AttachActorToActor _returnvalue self "None" "KeepWorld" "KeepWorld" "KeepWorld" true)
          (Default|DrawWire _returnvalue))))))

(fn SetasHead
  (Variables|Default|SetIsHeadNode true)
  (Rendering|Material|SetVectorParameterValueonMaterials (Variables|Default|GetWireNodeRoot) "Color" (Variables|Default|GetHeadColor)))

(fn SetasTail
  (Variables|Default|SetIsTailNode true)
  (Rendering|Material|SetVectorParameterValueonMaterials (Variables|Default|GetWireNodeRoot) "Color" (Variables|Default|GetTailColor))
  (bind _componentplacedon (Variables|Default|GetComponentPlacedOn)
    (:then
      (bind _asbp_part_interactive (Utilities|Casting|CastToBP_PartInteractive (Components|GetOwner _componentplacedon)))
      (Default|AddInputWire _asbp_part_interactive self))
    (:else)))

(fn AsPart
  (params (Conponent :type Primitive%20Component%20Object%20Reference))
  (bind _asbp_part (Utilities|Casting|CastToBP_Part (Components|GetOwner Conponent)))
  (return _asbp_part))

(fn AcceptsConnection
  (return (not (Utilities|IsValid (Variables|Default|GetPrevWireNode)))))

(fn RemoveNextConnection
  (params (NodeToRemove :type BP%20Wire%20Node%20Object%20Reference))
  (Utilities|Array|RemoveItem (Variables|Default|GetNextWireNodes) NodeToRemove))

(fn RemovePrevConnection
  (Variables|Default|SetPrevWireNode 0))

(fn RemoveWireNode
  (bind _componentplacedon (Variables|Default|GetComponentPlacedOn))
  (bind _part (CallFunction|AsInteractive _componentplacedon))
  (if (Variables|Default|GetIsTailNode)
    (Utilities|IsValid _part
      (:Is%20Valid
        (Default|RemoveParent _part self))
      (:Is%20Not%20Valid
        _)))
  (bind _prevwirenode (Variables|Default|GetPrevWireNode)
    (:then
      (CallFunction|RemoveNextConnection _prevwirenode self))
    (:else
      _))
  (for _array_element (Variables|Default|GetNextWireNodes)
    (Utilities|IsValid _array_element
      (:Is%20Valid
        (CallFunction|RemovePrevConnection _array_element))))
  (bind _componentplacedon_2 (Variables|Default|GetComponentPlacedOn)
    (:then
      (Default|RemoveWireNode (.GetBody (Default|GetBodyREF (CallFunction|AsPart _componentplacedon_2) _componentplacedon_2)) self))
    (:else
      _))
  (Actor|DestroyActor))

(fn AddNextConnection
  (params (NodeToAdd :type BP%20Wire%20Node%20Object%20Reference))
  (Utilities|Array|Add (Variables|Default|GetNextWireNodes) NodeToAdd))

(fn AddPrevConnection
  (params (NodeToAdd :type BP%20Wire%20Node%20Object%20Reference))
  (Variables|Default|SetPrevWireNode NodeToAdd))

(fn GetParentConnection
  (bind _prevwirenode (Variables|Default|GetPrevWireNode))
  (bind _componentplacedon (Variables|Default|GetComponentPlacedOn))
  (bind _wirenoderoot (Variables|Default|GetWireNodeRoot))
  (bind _wirenoderoot_2 (Variables|Default|GetWireNodeRoot))
  (bind _part (CallFunction|AsInteractive _componentplacedon))
  (if (Variables|Default|GetIsHeadNode)
    (Utilities|IsValid _part
      (:Is%20Valid
        (if (Variables|/Game/InventorySystem/Parts/Interactive/BP_PartInteractive.BP_PartInteractive_C|GetActive _part)
          (Rendering|Material|SetScalarParameterValueonMaterials _wirenoderoot_2 "Glow" 3.0)
          (else
            (Rendering|Material|SetScalarParameterValueonMaterials _wirenoderoot_2 "Glow" 0.5)))
        (return true _part))
      (:Is%20Not%20Valid
        _))
    (else
      (Utilities|IsValid _prevwirenode
        (:Is%20Valid
          (bind (_hasconnection _parentconnection) (CallFunction|GetParentConnection _prevwirenode))
          (if (Variables|/Game/InventorySystem/Parts/Interactive/BP_PartInteractive.BP_PartInteractive_C|GetActive _parentconnection)
            (Rendering|Material|SetScalarParameterValueonMaterials _wirenoderoot "Glow" 3.0)
            (else
              (Rendering|Material|SetScalarParameterValueonMaterials _wirenoderoot "Glow" 0.5)))
          (return _hasconnection _parentconnection))
        (:Is%20Not%20Valid
          _))))
  (return false 0))

(fn AsInteractive
  (params (Conponent :type Primitive%20Component%20Object%20Reference))
  (Utilities|IsValid Conponent
    (:Is%20Valid
      (bind _asbp_part_interactive (Utilities|Casting|CastToBP_PartInteractive (Components|GetOwner Conponent))
        (:then
          (return _asbp_part_interactive))
        (:CastFailed
          _)))
    (:Is%20Not%20Valid
      _))
  (return 0))