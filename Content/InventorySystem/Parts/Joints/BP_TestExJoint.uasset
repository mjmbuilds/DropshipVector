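; BP_TestExJoint is a test joint part in the inventory system that links several bodies with physics constraints.
; RepairJoint re-binds X, Y and X2 constraints from three outer bodies to the base body, and chains two of those outer bodies through a TransferBall via two further constraints.
; LockJoint and UnlockJoint switch only the X constraint's angular twist between locked and free; matching Y-constraint calls are left disconnected.
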(event EventBeginPlay
  (|CallParentFunction))

(event EventRepairJoint
  (Development|PrintString "Repair Constraint" true true "(R=0.000000,G=0.660000,B=1.000000,A=1.000000)" 1e+02)
  (Class|PhysicsConstraintComponent|SetConstrainedComponents (Variables|Default|GetJointConstraintX) (Variables|/Game/InventorySystem/Parts/BP_Body.BP_Body_C|GetBodyRoot (Utilities|Array|Get(acopy) (Variables|Default|GetBodies) 1)) "None" (Variables|/Game/InventorySystem/Parts/BP_Body.BP_Body_C|GetBodyRoot (Utilities|Array|Get(acopy) (Variables|Default|GetBodies))) "None")
  (Class|PhysicsConstraintComponent|SetConstrainedComponents (Variables|Default|GetJointConstraintY) (Variables|/Game/InventorySystem/Parts/BP_Body.BP_Body_C|GetBodyRoot (Utilities|Array|Get(acopy) (Variables|Default|GetBodies) 2)) "None" (Variables|/Game/InventorySystem/Parts/BP_Body.BP_Body_C|GetBodyRoot (Utilities|Array|Get(acopy) (Variables|Default|GetBodies))) "None")
  (Class|PhysicsConstraintComponent|SetConstrainedComponents (Variables|Default|GetJointConstraintX2) (Variables|/Game/InventorySystem/Parts/BP_Body.BP_Body_C|GetBodyRoot (Utilities|Array|Get(acopy) (Variables|Default|GetBodies) 3)) "None" (Variables|/Game/InventorySystem/Parts/BP_Body.BP_Body_C|GetBodyRoot (Utilities|Array|Get(acopy) (Variables|Default|GetBodies))) "None")
  (Class|PhysicsConstraintComponent|SetConstrainedComponents (Variables|Default|GetRoutConst1) (Variables|/Game/InventorySystem/Parts/BP_Body.BP_Body_C|GetBodyRoot (Utilities|Array|Get(acopy) (Variables|Default|GetBodies) 3)) "None" (Variables|Default|GetTransferBall) "None")
  (Class|PhysicsConstraintComponent|SetConstrainedComponents (Variables|Default|GetRoutConst2) (Variables|Default|GetTransferBall) "None" (Variables|/Game/InventorySystem/Parts/BP_Body.BP_Body_C|GetBodyRoot (Utilities|Array|Get(acopy) (Variables|Default|GetBodies) 1)) "None"))

(event EventUnlockJoint
  (Class|PhysicsConstraintComponent|SetAngularTwistLimit (Variables|Default|GetJointConstraintX) "ACM_Free" 0.0))

(event EventLockJoint
  (Class|PhysicsConstraintComponent|SetAngularTwistLimit (Variables|Default|GetJointConstraintX) "ACM_Locked" 0.0))

(fn ConstructionScript
  (|CallParentFunction))