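; Test joint part for the inventory build system that simulates a gear reduction between two physics joint ends.
; Outside build mode, each Tick sets both ends' angular velocities from their averaged spin, scaled up for one and down for the other.
; Lock, unlock and repair events switch twist limits on two constraints or reattach them to three bodies, the first shared.
; Unconnected impulse and torque nodes never run.
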(event EventBeginPlay
  (|CallParentFunction))

(event EventTick
  (params (DeltaSeconds :type Float%20%28single-precision%29))
  (bind _jointend2 (Variables|Default|GetJointEnd2))
  (bind _jointend1 (Variables|Default|GetJointEnd1))
  (bind _returnvalue (Physics|GetPhysicsAngularVelocityinDegrees _jointend1 "None"))
  (bind _returnvalue_2 (Physics|GetPhysicsAngularVelocityinDegrees _jointend2 "None"))
  (bind _returnvalue_3 (+ _returnvalue _returnvalue_2))
  (bind _returnvalue_4 (/ _returnvalue_3 2.0))
  (|CallParentFunction DeltaSeconds)
  (if (not (Variables|Default|GetInBuildMode))
    (Class|PrimitiveComponent|SetAllPhysicsAngularVelocityinDegrees (Variables|Default|GetJointEnd1) (* _returnvalue_4 1.5) false)
    (Class|PrimitiveComponent|SetAllPhysicsAngularVelocityinDegrees (Variables|Default|GetJointEnd2) (* _returnvalue_4 0.5) false)))

(event EventRepairJoint
  (Development|PrintString "Repair Constraint" true true "(R=0.000000,G=0.660000,B=1.000000,A=1.000000)" 1e+02)
  (Class|PhysicsConstraintComponent|SetConstrainedComponents (Variables|Default|GetJointConstraint1) (Variables|/Game/InventorySystem/Parts/BP_Body.BP_Body_C|GetBodyRoot (Utilities|Array|Get(acopy) (Variables|Default|GetBodies) 1)) "None" (Variables|/Game/InventorySystem/Parts/BP_Body.BP_Body_C|GetBodyRoot (Utilities|Array|Get(acopy) (Variables|Default|GetBodies))) "None")
  (Class|PhysicsConstraintComponent|SetConstrainedComponents (Variables|Default|GetJointConstraint2) (Variables|/Game/InventorySystem/Parts/BP_Body.BP_Body_C|GetBodyRoot (Utilities|Array|Get(acopy) (Variables|Default|GetBodies) 2)) "None" (Variables|/Game/InventorySystem/Parts/BP_Body.BP_Body_C|GetBodyRoot (Utilities|Array|Get(acopy) (Variables|Default|GetBodies))) "None"))

(event EventUnlockJoint
  (Class|PhysicsConstraintComponent|SetAngularTwistLimit (Variables|Default|GetJointConstraint1) "ACM_Free" 0.0)
  (Class|PhysicsConstraintComponent|SetAngularTwistLimit (Variables|Default|GetJointConstraint2) "ACM_Free" 0.0))

(event EventLockJoint
  (Class|PhysicsConstraintComponent|SetAngularTwistLimit (Variables|Default|GetJointConstraint1) "ACM_Locked" 0.0)
  (Class|PhysicsConstraintComponent|SetAngularTwistLimit (Variables|Default|GetJointConstraint2) "ACM_Locked" 0.0))

(fn ConstructionScript
  (|CallParentFunction))