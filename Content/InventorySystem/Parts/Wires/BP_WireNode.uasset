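; BP_WireNode is one node in a player-placed wire chain on parts, linking a source part to the interactive part under the tail node as its parent.
; Connection attempts and green/no-connection coloring propagate recursively along the doubly linked Prev/Next nodes.
; Segments on the same body use a stretched mesh; across bodies, a runtime cable component follows and breaks beyond max length.
; Removal clears links, connection and body registration.
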(event EventTick
  (params (DeltaSeconds :type Float%20%28single-precision%29))
  (bind _cable (Variables|Default|GetCable))
  (bind _nextwirenode (Variables|Default|GetNextWireNode))
  (bind _returnvalue (Transformation|GetActorLocation _nextwirenode))
  (Utilities|IsValid (Variables|Default|GetComponentPlacedOn)
    (:Is%20Valid
      (Utilities|IsValid _cable
        (:Is%20Valid
          (Variables|/Script/CableComponent.CableComponent|SetEndLocation _cable (Math|Transform|InverseTransformLocation (Transformation|GetActorTransform) _returnvalue))
          (if (> (Math|Vector|VectorLength (- _returnvalue (Transformation|GetActorLocation))) (Variables|Default|GetMaxWireLength))
            (CallFunction|BreakCable)))))
    (:Is%20Not%20Valid
      (Actor|DestroyActor))))

(event EventEndPlay
  (params (EndPlayReason :type EEndPlayReason%20Enum :default "Destroyed"))
  (bind _componentplacedon (Variables|Default|GetComponentPlacedOn))
  (CallFunction|RemovePrevWire)
  (CallFunction|RemoveConnection)
  (CallFunction|RevSetConnectionBad)
  (CallFunction|FwdSetConnectionBad)
  (CallFunction|RemoveSelffromNeighbors)
  (Utilities|IsValid _componentplacedon
    (:Is%20Valid
      (Default|RemoveWireNode (.GetBody (Default|GetBodyREF (CallFunction|AsPart _componentplacedon) _componentplacedon)) self))))

(event EventBeginPlay
  (bind _noconnectioncolor (Variables|Default|GetNoConnectionColor))
  (Rendering|Material|SetVectorParameterValueonMaterials (Variables|Default|GetWireNode) "Color" _noconnectioncolor)
  (Rendering|Material|SetVectorParameterValueonMaterials (Variables|Default|GetWire) "Color" _noconnectioncolor))

(fn ConstructionScript
  (|CallParentFunction))

(fn RemoveConnection
  (bind _nextwirenode (Variables|Default|GetNextWireNode))
  (if (Variables|Default|GetIsTailNode)
    (Default|RemoveParent (CallFunction|AsInteractive (Variables|Default|GetComponentPlacedOn)) (Variables|Default|GetPartForConnection))
    (else
      (Utilities|IsValid _nextwirenode
        (:Is%20Valid
          (CallFunction|RemoveConnection _nextwirenode)))))
  (Variables|Default|SetPartForConnection 0))

(fn DrawWire
  (bind _returnvalue (Transformation|GetActorLocation))
  (bind _nextwirenode (Variables|Default|GetNextWireNode))
  (bind _nextwirenode_2 (Variables|Default|GetNextWireNode))
  (bind _wire (Variables|Default|GetWire))
  (bind _wire_2 (Variables|Default|GetWire))
  (bind _componentplacedon (Variables|Default|GetComponentPlacedOn))
  (bind _wire_3 (Variables|Default|GetWire))
  (bind _returnvalue_2 (Transformation|GetActorLocation _nextwirenode))
  (bind _componentplacedon_2 (Variables|BP_WireNode_C|GetComponentPlacedOn _nextwirenode_2))
  (bind _returnvalue_3 (- _returnvalue _returnvalue_2))
  (Utilities|IsValid _nextwirenode_2
    (:Is%20Valid
      (Utilities|IsValid _componentplacedon
        (:Is%20Valid
          (Utilities|IsValid _componentplacedon_2
            (:Is%20Valid
              (if (== (.GetBody (Default|GetBodyREF (CallFunction|AsPart _componentplacedon) _componentplacedon)) (.GetBody (Default|GetBodyREF (CallFunction|AsPart _componentplacedon_2) _componentplacedon_2)))
                (Transformation|SetWorldLocationAndRotation _wire_2 (/ (+ _returnvalue _returnvalue_2) 2.0) (Math|Conversions|RotationFromXVector _returnvalue_3) false true)
                (Transformation|SetRelativeScale3D _wire_2 (Math|Vector|MakeVector (Math|Float|Max(Float) (/ (Math|Vector|VectorLength _returnvalue_3) 2e+01) 0.1) 0.75 0.75))
                (else
                  (bind _returnvalue_4 (AddComponent|AddCableComponent false (Math|Transform|MakeTransform "0, 0, 0")))
                  (bind _output_get (Variables|Default|SetCable _returnvalue_4))
                  (Variables|/Script/CableComponent.CableComponent|SetbEnableStiffness _output_get true)
                  (Rendering|Material|SetMaterial _output_get 0 "/Game/Materials/M_Plastic_Inst.M_Plastic_Inst")
                  (Rendering|Material|SetVectorParameterValueonMaterials _output_get "Color" (Variables|Default|GetNoConnectionColor))
                  (Class|PrimitiveComponent|SetPhysMaterialOverride _output_get "/Game/PhysicsMaterials/PM_Data.PM_Data")
                  (Variables|/Script/CableComponent.CableComponent|SetCableLength _output_get (Math|Vector|VectorLength (- (Transformation|GetActorLocation (Variables|Default|GetNextWireNode)) (Transformation|GetActorLocation))))
                  (Variables|/Script/CableComponent.CableComponent|SetCableWidth _output_get 3.0)
                  (Transformation|SetWorldLocation _wire_3 (Transformation|GetActorLocation) false true)
                  (Transformation|SetRelativeScale3D _wire_3 "0.100000,0.750000,0.750000"))))))))
    (:Is%20Not%20Valid
      (Transformation|SetWorldLocation _wire (Transformation|GetActorLocation) false true)
      (Transformation|SetRelativeScale3D _wire "0.100000,0.750000,0.750000")
      (Utilities|IsValid (Variables|Default|GetCable)
        (:Is%20Valid
          (Components|DestroyComponent (Variables|Default|GetCable)))))))

(fn RemovePrevWire
  (bind _prevwirenode (Variables|Default|GetPrevWireNode))
  (Utilities|IsValid _prevwirenode
    (:Is%20Valid
      (CallFunction|ResetWire _prevwirenode))))

(fn ResetWire
  (Variables|Default|SetNextWireNode 0)
  (CallFunction|DrawWire))

(fn SetasHead
  (Variables|Default|SetIsHeadNode true)
  (Rendering|Material|SetVectorParameterValueonMaterials (Variables|Default|GetWireNode) "Color" (Variables|Default|GetHeadColor)))

(fn SetasTail
  (Variables|Default|SetIsTailNode true)
  (Rendering|Material|SetVectorParameterValueonMaterials (Variables|Default|GetWireNode) "Color" (Variables|Default|GetTailColor)))

(fn RevSetConnectionBad
  (bind _noconnectioncolor (Variables|Default|GetNoConnectionColor))
  (bind _prevwirenode (Variables|Default|GetPrevWireNode))
  (bind _cable (Variables|Default|GetCable))
  (Rendering|Material|SetVectorParameterValueonMaterials (Variables|Default|GetWire) "Color" _noconnectioncolor)
  (Utilities|IsValid _cable
    (:Is%20Valid
      (Rendering|Material|SetVectorParameterValueonMaterials _cable "Color" _noconnectioncolor))
    (:Is%20Not%20Valid
      _))
  (if (Math|Boolean|NORBoolean (Variables|Default|GetIsHeadNode) (Variables|Default|GetIsTailNode))
    (Rendering|Material|SetVectorParameterValueonMaterials (Variables|Default|GetWireNode) "Color" _noconnectioncolor))
  (Utilities|IsValid _prevwirenode
    (:Is%20Valid
      (CallFunction|RevSetConnectionBad _prevwirenode))))

(fn RevSetConnectionGood
  (bind _goodconnectioncolor (Variables|Default|GetGoodConnectionColor))
  (bind _prevwirenode (Variables|Default|GetPrevWireNode))
  (bind _cable (Variables|Default|GetCable))
  (Rendering|Material|SetVectorParameterValueonMaterials (Variables|Default|GetWire) "Color" _goodconnectioncolor)
  (Utilities|IsValid _cable
    (:Is%20Valid
      (Rendering|Material|SetVectorParameterValueonMaterials _cable "Color" _goodconnectioncolor))
    (:Is%20Not%20Valid
      _))
  (if (Math|Boolean|NORBoolean (Variables|Default|GetIsHeadNode) (Variables|Default|GetIsTailNode))
    (Rendering|Material|SetVectorParameterValueonMaterials (Variables|Default|GetWireNode) "Color" _goodconnectioncolor))
  (Utilities|IsValid _prevwirenode
    (:Is%20Valid
      (CallFunction|RevSetConnectionGood _prevwirenode))))

(fn FwdSetConnectionBad
  (bind _noconnectioncolor (Variables|Default|GetNoConnectionColor))
  (bind _nextwirenode (Variables|Default|GetNextWireNode))
  (bind _cable (Variables|Default|GetCable))
  (Rendering|Material|SetVectorParameterValueonMaterials (Variables|Default|GetWire) "Color" _noconnectioncolor)
  (Utilities|IsValid _cable
    (:Is%20Valid
      (Rendering|Material|SetVectorParameterValueonMaterials _cable "Color" _noconnectioncolor))
    (:Is%20Not%20Valid
      _))
  (if (Math|Boolean|NORBoolean (Variables|Default|GetIsHeadNode) (Variables|Default|GetIsTailNode))
    (Rendering|Material|SetVectorParameterValueonMaterials (Variables|Default|GetWireNode) "Color" _noconnectioncolor))
  (Utilities|IsValid _nextwirenode
    (:Is%20Valid
      (CallFunction|FwdSetConnectionBad _nextwirenode))))

(fn FwdSetConnectionGood
  (bind _goodconnectioncolor (Variables|Default|GetGoodConnectionColor))
  (bind _nextwirenode (Variables|Default|GetNextWireNode))
  (bind _cable (Variables|Default|GetCable))
  (Rendering|Material|SetVectorParameterValueonMaterials (Variables|Default|GetWire) "Color" _goodconnectioncolor)
  (Utilities|IsValid _cable
    (:Is%20Valid
      (Rendering|Material|SetVectorParameterValueonMaterials _cable "Color" _goodconnectioncolor))
    (:Is%20Not%20Valid
      _))
  (if (Math|Boolean|NORBoolean (Variables|Default|GetIsHeadNode) (Variables|Default|GetIsTailNode))
    (Rendering|Material|SetVectorParameterValueonMaterials (Variables|Default|GetWireNode) "Color" _goodconnectioncolor))
  (Utilities|IsValid _nextwirenode
    (:Is%20Valid
      (CallFunction|FwdSetConnectionGood _nextwirenode))))

(fn RemoveSelffromNeighbors
  (Utilities|IsValid (Variables|Default|GetPrevWireNode)
    (:Is%20Valid
      (Variables|BP_WireNode_C|SetNextWireNode (Variables|Default|GetPrevWireNode) 0))
    (:Is%20Not%20Valid
      _))
  (Utilities|IsValid (Variables|Default|GetNextWireNode)
    (:Is%20Valid
      (Variables|BP_WireNode_C|SetPrevWireNode (Variables|Default|GetNextWireNode) 0))))

(fn TryConnection
  (bind _nextwirenode (Variables|Default|GetNextWireNode))
  (bind _componentplacedon (Variables|Default|GetComponentPlacedOn))
  (Utilities|IsValid (Variables|Default|GetPartForConnection)
    (:Is%20Valid
      (if (Variables|Default|GetIsTailNode)
        (Utilities|IsValid _componentplacedon
          (:Is%20Valid
            (Default|AddParent (CallFunction|AsInteractive _componentplacedon) (Variables|Default|GetPartForConnection))
            (CallFunction|RevSetConnectionGood)))
        (else
          (Utilities|IsValid _nextwirenode
            (:Is%20Valid
              (Variables|BP_WireNode_C|SetPartForConnection _nextwirenode (Variables|Default|GetPartForConnection))
              (CallFunction|TryConnection _nextwirenode))))))))

(fn AsPart
  (params (Conponent :type Primitive%20Component%20Object%20Reference))
  (bind _asbp_part (Utilities|Casting|CastToBP_Part (Components|GetOwner Conponent)))
  (return _asbp_part))

(fn AsInteractive
  (params (Component :type Primitive%20Component%20Object%20Reference))
  (bind _asbp_part_interactive (Utilities|Casting|CastToBP_PartInteractive (Components|GetOwner Component)))
  (return _asbp_part_interactive))

(fn DrawPlacementWire
  (params (Location :type Vector))
  (bind _returnvalue (Transformation|GetActorLocation))
  (bind _wire (Variables|Default|GetWire))
  (bind _returnvalue_2 (- _returnvalue Location))
  (Transformation|SetWorldLocationAndRotation _wire (/ (+ Location _returnvalue) 2.0) (Math|Conversions|RotationFromXVector _returnvalue_2) false true)
  (Transformation|SetRelativeScale3D _wire (Math|Vector|MakeVector (Math|Float|Max(Float) (/ (Math|Vector|VectorLength _returnvalue_2) 2e+01) 0.1) 0.75 0.75)))

(fn AcceptingWires
  (return (not (Utilities|IsValid (Variables|Default|GetPrevWireNode))) (not (Utilities|IsValid (Variables|Default|GetNextWireNode)))))

(fn BreakCable
  (bind _cable (Variables|Default|GetCable))
  (CallFunction|RemoveConnection)
  (CallFunction|RevSetConnectionBad)
  (CallFunction|FwdSetConnectionBad)
  (Variables|Default|SetNextWireNode 0)
  (Utilities|IsValid _cable
    (:Is%20Valid
      (Components|DestroyComponent _cable))))