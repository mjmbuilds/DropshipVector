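; BP_BreakoutDriverSeat_Power is an interactive electronics part that outputs the throttled power of a connected driver seat.
; Each tick, if it has a parent, it follows its first input wire to that wire's parent connection and casts it to BP_DriverSeat.
; It copies the seat's ThrottledPower into Power and brightens or dims the LogicBoxDisplay Glow material parameter by whether power is nonzero.
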(event EventTick
  (params (DeltaSeconds :type Float%20%28single-precision%29))
  (bind _logicboxdisplay (Variables|Default|GetLogicBoxDisplay))
  (bind _inputwires (Variables|Default|GetInputWires))
  (bind _output (Utilities|Array|Get(acopy) _inputwires))
  (|CallParentFunction DeltaSeconds)
  (if (CallFunction|HasAnyParent)
    (Utilities|IsValid _output
      (:Is%20Valid
        (bind (_hasconnection _parentconnection) (Default|GetParentConnection _output))
        (if _hasconnection
          (bind _asbp_driver_seat (Utilities|Casting|CastToBP_DriverSeat _parentconnection))
          (bind _output_get (Variables|Default|SetPower (Variables|/Game/InventorySystem/Parts/Interactive/Seats/BP_DriverSeat.BP_DriverSeat_C|GetThrottledPower _asbp_driver_seat)))
          (if (!= _output_get 0.0)
            (Rendering|Material|SetScalarParameterValueonMaterials _logicboxdisplay "Glow" 3.0)
            (else
              (Rendering|Material|SetScalarParameterValueonMaterials _logicboxdisplay "Glow" 0.5))))))))

(fn ConstructionScript
  (|CallParentFunction))