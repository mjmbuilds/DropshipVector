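; BP_Motor is an interactive motor part for player creations that spins a joint between two bodies using a physics constraint.
; Each tick outside stasis, the first parent's Power times EngineSpeed sets the angular velocity target, with EngineStrength as drive strength.
; On stopping, it enables twist orientation drive targeting the constraint's relative roll.
; Events lock or free the twist axis and reconnect the bodies for repair.
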(event EventTick
  (params (DeltaSeconds :type Float%20%28single-precision%29))
  (bind _enginespeed (Variables|Default|GetEngineSpeed))
  (bind _parents (Variables|Default|GetParents))
  (bind _engineconstraint (Variables|Default|GetEngineConstraint))
  (bind _output (Utilities|Array|Get(acopy) _parents))
  (bind _power (Variables|/Game/InventorySystem/Parts/Interactive/BP_PartInteractive.BP_PartInteractive_C|GetPower _output))
  (bind _returnvalue (* _power _enginespeed))
  (|CallParentFunction DeltaSeconds)
  (if (CallFunction|HasAnyParent)
    (Utilities|IsValid _output
      (:Is%20Valid
        (if (not (Variables|/Game/InventorySystem/Parts/BP_Creation.BP_Creation_C|GetInStasis (Variables|Default|GetCreation)))
          (Class|PhysicsConstraintComponent|SetAngularVelocityTarget _engineconstraint (Math|Vector|MakeVector _returnvalue 0.0 0.0))
          (Class|PhysicsConstraintComponent|SetAngularDriveParams _engineconstraint 0.0 (Variables|Default|GetEngineStrength) 0.0)
          (if (== _returnvalue 0.0)
            (if (Variables|Default|GetTempWasMoving)
              (Variables|Default|SetTempWasMoving false)
              (Class|PhysicsConstraintComponent|SetOrientationDriveTwistandSwing _engineconstraint true false)
              (Class|PhysicsConstraintComponent|SetAngularOrientationTarget _engineconstraint (Math|Rotator|MakeRotator (.roll (Variables|/Script/Engine.SceneComponent|GetRelativeRotation _engineconstraint)) 0.0 0.0)))
            (else
              (Variables|Default|SetTempWasMoving true)
              (Class|PhysicsConstraintComponent|SetOrientationDriveTwistandSwing _engineconstraint false false))))))))

(event EventUnlockJoint
  (Class|PhysicsConstraintComponent|SetAngularTwistLimit (Variables|Default|GetEngineConstraint) "ACM_Free" 0.0))

(event EventLockJoint
  (Class|PhysicsConstraintComponent|SetAngularTwistLimit (Variables|Default|GetEngineConstraint) "ACM_Locked" 0.0)
  (Class|PrimitiveComponent|WakeAllRigidBodies (CallFunction|AsPrimitive (Variables|Transformation|GetRootComponent self))))

(event EventRepairJoint
  (Class|PhysicsConstraintComponent|SetConstrainedComponents (Variables|Default|GetEngineConstraint) (Variables|/Game/InventorySystem/Parts/BP_Body.BP_Body_C|GetBodyRoot (Utilities|Array|Get(acopy) (Variables|Default|GetBodies) 1)) "None" (Variables|/Game/InventorySystem/Parts/BP_Body.BP_Body_C|GetBodyRoot (Utilities|Array|Get(acopy) (Variables|Default|GetBodies))) "None"))

(fn ConstructionScript
  (|CallParentFunction))