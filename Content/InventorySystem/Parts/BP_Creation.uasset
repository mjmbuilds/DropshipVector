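; BP_Creation is a manager actor for a player creation, grouping bodies whose members are BP_Part actors.
; It keeps a unique Bodies list, forwards stasis, physics, ungrounding, teleport, wire redraw and deletion to each, and destroys itself on Tick when empty unless disabled.
; Shattering detaches every part, applies random impulses, optionally sets randomized destroy timers, then destroys the bodies and itself.
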(event EventBeginPlay
  ;[1 1 1] Debug
  (Development|PrintString (Utilities|String|Append (Utilities|GetDisplayName self) " Created") true true "(R=0.500000,G=0.000000,B=1.000000,A=1.000000)" 1e+02))

(event EventEndPlay
  (params (EndPlayReason :type EEndPlayReason%20Enum :default "Destroyed"))
  ;[1 1 1] Debug
  (Development|PrintString (Utilities|String|Append (Utilities|GetDisplayName self) " was Destroyed") true true "(R=0.250000,G=0.000000,B=0.500000,A=1.000000)" 1e+02))

(event EventTick
  (params (DeltaSeconds :type Float%20%28single-precision%29))
  (if (< (Utilities|Array|Length (Variables|Default|GetBodies)) 1)
    (if (not (Variables|Default|GetDisableDestroy))
      (Actor|DestroyActor))))

(fn ConstructionScript)

(fn AddBody
  (params (BodyToAdd :type BP%20Body%20Object%20Reference))
  (Utilities|Array|AddUnique (Variables|Default|GetBodies) BodyToAdd))

(fn RemoveBody
  (params (BodyToRemove :type BP%20Body%20Object%20Reference))
  (Utilities|Array|RemoveItem (Variables|Default|GetBodies) BodyToRemove))

(fn GetAllMembers
  (for _array_element (Variables|Default|GetBodies)
    (for _array_element_2 (Variables|/Game/InventorySystem/Parts/BP_Body.BP_Body_C|GetMembers _array_element)
      (Utilities|Array|AddUnique (LocalVariables|GetReturnParts) (CallFunction|AsPart _array_element_2))))
  (return (LocalVariables|GetReturnParts)))

(fn ShatterCreation
  (params (DestroyParts :type Boolean))
  (bind _allparts (CallFunction|GetAllMembers))
  (for _array_element _allparts
    (Variables|/Game/InventorySystem/Parts/BP_Part.BP_Part_C|SetCreation _array_element 0)
    (Variables|/Game/InventorySystem/Parts/BP_Part.BP_Part_C|SetBodies _array_element (LocalVariables|GetEmptyBodies))
    (Transformation|DetachFromComponent (Variables|/Script/Engine.Actor|GetRootComponent _array_element) "KeepWorld" "KeepWorld" "KeepWorld" true)
    (Physics|SetSimulatePhysics (CallFunction|AsPrimitive (Variables|/Script/Engine.Actor|GetRootComponent _array_element)) true)
    (Physics|AddImpulseatLocation (CallFunction|AsPrimitive (Variables|/Script/Engine.Actor|GetRootComponent _array_element)) (* (Math|Random|RandomUnitVector) (LocalVariables|GetShatterForce)) (Transformation|GetActorLocation _array_element) "None")
    (if DestroyParts
      (Variables|/Game/InventorySystem/Parts/BP_Part.BP_Part_C|SetDestroyTimer _array_element (+ (Math|Random|RandomInteger 150) 50))))
  (bind _output_get (LocalVariables|SetTempBodies (Variables|Default|GetBodies)))
  (for _array_element_2 _output_get
    (Actor|DestroyActor _array_element_2))
  (Actor|DestroyActor))

(fn AsPart
  (params (Component :type Primitive%20Component%20Object%20Reference))
  (bind _asbp_part (Utilities|Casting|CastToBP_Part (Components|GetOwner Component)))
  (return _asbp_part))

(fn EndStasis
  (Variables|Default|SetInStasis false)
  (for _array_element (Variables|Default|GetBodies)
    (Default|EndStasis _array_element)))

(fn BeginStasis
  (Variables|Default|SetInStasis true)
  (for _array_element (Variables|Default|GetBodies)
    (Default|BeginStasis _array_element)))

(fn UngroundCreation
  (for _array_element (Variables|Default|GetBodies)
    (Default|Unground _array_element)))

(fn EnablePhysics
  (for _array_element (Variables|Default|GetBodies)
    (Physics|SetSimulatePhysics (Variables|/Game/InventorySystem/Parts/BP_Body.BP_Body_C|GetBodyRoot _array_element) true)))

(fn DisablePhysics
  (for _array_element (Variables|Default|GetBodies)
    (Physics|SetSimulatePhysics (Variables|/Game/InventorySystem/Parts/BP_Body.BP_Body_C|GetBodyRoot _array_element) false)))

(fn TeleportOffset
  (params (OffsetVector :type Vector))
  (for _array_element (Variables|Default|GetBodies)
    (Utilities|IsValid _array_element
      (:Is%20Valid
        (Transformation|SetWorldLocation (Variables|/Script/Engine.Actor|GetRootComponent _array_element) (+ (Transformation|GetActorLocation _array_element) OffsetVector) false true)))))

(fn AsPrimitive
  (params (ActComp :type Actor%20Component%20Object%20Reference))
  (bind _asprimitive_component (Utilities|Casting|CastToPrimitiveComponent ActComp))
  (return _asprimitive_component))

(fn GetAllWires
  (bind _allwirenodes (LocalVariables|GetAllWireNodes))
  (for _array_element (Variables|Default|GetBodies)
    (for _array_element_2 (Variables|/Game/InventorySystem/Parts/BP_Body.BP_Body_C|GetWireNodes _array_element)
      (Utilities|Array|Add _allwirenodes _array_element_2)
      (return _allwirenodes))))

(fn DeleteCreation
  (for _array_element (Variables|Default|GetBodies)
    (Default|DeleteBody _array_element))
  (Actor|DestroyActor))

(fn RedrawAllWires
  (for _array_element (Variables|Default|GetBodies)
    (Default|RedrawAllWires _array_element)))