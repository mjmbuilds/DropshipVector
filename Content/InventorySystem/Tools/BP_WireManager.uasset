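; BP_WireManager is the build tool for placing, chaining and removing wires on parts.
; A camera line trace classifies the hit as node, wire or part, checking build range and wire length.
; Placing links existing nodes or spawns attached ones, marking head or tail nodes on interactive parts and registering tails as parents.
; While placing, Tick updates a stretched preview wire and node, tinted by placement validity.
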(event Custom|PlaceWire
  (CallFunction|UpdateTrace)
  (if (Variables|Default|GetCanPlace)
    (Utilities|IsValid (Variables|Default|GetHitWireNode)
      (:Is%20Valid
        (if (Variables|Default|GetIsPlacing)
          (CallFunction|ConnecttoNode)
          (else
            (Variables|Default|SetIsPlacing true)
            (Variables|Default|SetFromNode (Variables|Default|GetHitWireNode)))))
      (:Is%20Not%20Valid
        (Utilities|IsValid (Variables|Default|GetHitPart)
          (:Is%20Valid
            (CallFunction|PlaceNewWireNode)))))))

(event Custom|RemoveWire
  (bind _hitwirenode (Variables|Default|GetHitWireNode))
  (bind _hitwire (Variables|Default|GetHitWire))
  (if (Variables|Default|GetIsPlacing)
    (CallFunction|CancelPlacing)
    (else
      (CallFunction|UpdateTrace)
      (Utilities|IsValid _hitwirenode
        (:Is%20Valid
          (Default|RemoveWireNode _hitwirenode))
        (:Is%20Not%20Valid
          (Utilities|IsValid _hitwire
            (:Is%20Valid
              (Default|RemoveWire _hitwire))))))))

(event EventTick
  (params (DeltaSeconds :type Float%20%28single-precision%29))
  (if (Variables|Default|GetIsPlacing)
    (Utilities|IsValid (Variables|Default|GetFromNode)
      (:Is%20Valid
        (CallFunction|UpdateTrace)
        (CallFunction|DrawPlacementWire))
      (:Is%20Not%20Valid
        (Variables|Default|SetIsPlacing false)
        (CallFunction|HidePlacementWire)))))

(fn ConstructionScript)

(fn UpdateTrace
  (bind _player (Variables|Default|GetPlayer))
  (bind _player_2 (Variables|Default|GetPlayer))
  (bind _buildrange (Variables|/Game/FirstPersonBP/FirstPersonCharacter.FirstPersonCharacter_C|GetBuildRange _player))
  (bind _firstpersoncamera (Variables|/Game/FirstPersonBP/FirstPersonCharacter.FirstPersonCharacter_C|GetFirstPersonCamera _player_2))
  (bind _returnvalue (Transformation|GetWorldLocation _firstpersoncamera))
  (bind _returnvalue_2 (Math|Vector|GetForwardVector _firstpersoncamera))
  (bind _returnvalue_3 (* _returnvalue_2 _buildrange))
  (bind _returnvalue_4 (+ _returnvalue _returnvalue_3))
  (bind (_outhit _returnvalue_5) (Collision|LineTraceByChannel _returnvalue _returnvalue_4 "TraceTypeQuery1" false (Utilities|Array|MakeArray (Variables|Default|GetFromNode) (Variables|Default|GetPlayer)) "None"))
  (bind _output_get (Variables|Default|SetTraceHit _returnvalue_5))
  (if _output_get
    (bind _output_get_2 (Variables|Default|SetTraceEndLocation (.ImpactPoint (Collision|BreakHitResult _outhit))))
    (Variables|Default|SetHitNormal (.ImpactNormal (Collision|BreakHitResult _outhit)))
    (bind _fromnode (Variables|Default|GetFromNode)
      (:then
        (if (< (Math|Vector|VectorLength (- (Transformation|GetActorLocation _fromnode) _output_get_2)) (Variables|Default|GetMaxWireLength))
          (bind _asbp_wire_node (Utilities|Casting|CastToBP_WireNode (.HitActor (Collision|BreakHitResult _outhit)) :!label _label)
            (:then
              (Variables|Default|SetHitWireNode _asbp_wire_node)
              (Variables|Default|SetHitWire 0)
              (Variables|Default|SetHitPart 0)
              (Variables|Default|SetHitComponent 0)
              (if (Variables|Default|GetIsPlacing)
                (bind _acceptsprev (Default|AcceptsConnection _asbp_wire_node))
                (if _acceptsprev
                  (CallFunction|SetCanPlace true)
                  (else
                    (CallFunction|SetCanPlace false)))
                (else
                  (CallFunction|SetCanPlace true))))
            (:CastFailed
              (Variables|Default|SetHitWireNode 0)
              (bind _asbp_wire (Utilities|Casting|CastToBP_Wire (.HitActor (Collision|BreakHitResult _outhit)))
                (:then
                  (Variables|Default|SetHitWire _asbp_wire)
                  (Variables|Default|SetHitPart 0)
                  (Variables|Default|SetHitComponent 0)
                  (CallFunction|SetCanPlace false))
                (:CastFailed
                  (Variables|Default|SetHitWire 0)
                  (bind _asbp_part (Utilities|Casting|CastToBP_Part (.HitActor (Collision|BreakHitResult _outhit)))
                    (:then
                      (Variables|Default|SetHitPart _asbp_part)
                      (Variables|Default|SetHitComponent (.HitComponent (Collision|BreakHitResult _outhit)))
                      (CallFunction|SetCanPlace true))
                    (:CastFailed
                      (Variables|Default|SetHitPart 0)
                      (Variables|Default|SetHitComponent 0)
                      (CallFunction|SetCanPlace false)))))))
          (else
            (CallFunction|SetCanPlace false))))
      (:else
        (goto _label)))
    (else
      (Variables|Default|SetTraceEndLocation _returnvalue_4)
      (CallFunction|SetCanPlace false))))

(fn CancelPlacing
  (Variables|Default|SetIsPlacing false)
  (CallFunction|HidePlacementWire)
  (Variables|Default|SetFromNode 0))

(fn ConnecttoNode
  (bind _hitwirenode (Variables|Default|GetHitWireNode))
  (bind _fromnode (Variables|Default|GetFromNode))
  (Default|AddNextConnection _fromnode _hitwirenode)
  (Default|AddPrevConnection _hitwirenode _fromnode)
  (Default|DrawWires _fromnode)
  (CallFunction|CancelPlacing))

(fn PlaceNewWireNode
  (bind _returnvalue (Game|SpawnActorfromClass "/Game/InventorySystem/Wires/BP_WireNode.BP_WireNode_C" (Math|Transform|MakeTransform (Variables|Default|GetTraceEndLocation) (Math|Rotator|MakeRotfromZ (Variables|Default|GetHitNormal))) "Undefined" 0 (Variables|Default|GetHitComponent) 0))
  (bind _output_get (LocalVariables|SetPlacedNode _returnvalue))
  (Default|AddWireNode (.GetBody (Default|GetBodyREF (Variables|Default|GetHitPart) (Variables|Default|GetHitComponent))) _output_get)
  (Transformation|AttachComponentToComponent (Variables|/Script/Engine.Actor|GetRootComponent _output_get) (Variables|Default|GetHitComponent) "None" "KeepWorld" "KeepWorld" "KeepWorld" true)
  (if (Variables|Default|GetIsPlacing)
    (Utilities|IsValid (Variables|Default|GetFromNode)
      (:Is%20Valid
        (Default|AddNextConnection (Variables|Default|GetFromNode) (LocalVariables|GetPlacedNode))
        (Default|AddPrevConnection (LocalVariables|GetPlacedNode) (Variables|Default|GetFromNode))
        (Default|DrawWires (Variables|Default|GetFromNode)))
      (:Is%20Not%20Valid
        _)))
  (bind _asbp_part_interactive (Utilities|Casting|CastToBP_PartInteractive (Variables|Default|GetHitPart))
    (:then
      (if (Variables|Default|GetIsPlacing)
        (if (Default|CanAcceptParent _asbp_part_interactive)
          (Default|SetasTail (LocalVariables|GetPlacedNode))
          (Variables|Default|SetIsPlacing false)
          (Variables|Default|SetFromNode 0)
          (Utilities|IsValid (CallFunction|AsInteractive (Variables|/Game/InventorySystem/Wires/BP_WireNode.BP_WireNode_C|GetComponentPlacedOn (LocalVariables|GetPlacedNode)))
            (:Is%20Valid
              (Default|AddParent (CallFunction|AsInteractive (Variables|/Game/InventorySystem/Wires/BP_WireNode.BP_WireNode_C|GetComponentPlacedOn (LocalVariables|GetPlacedNode))) (LocalVariables|GetPlacedNode))))
          (else
            (Variables|Default|SetFromNode (LocalVariables|GetPlacedNode) :!label _label)
            (Variables|Default|SetIsPlacing true)))
        (else
          (Default|SetasHead (LocalVariables|GetPlacedNode))
          (goto _label))))
    (:CastFailed
      (goto _label))))

(fn DrawPlacementWire
  (bind _fromnode (Variables|Default|GetFromNode))
  (bind _traceendlocation (Variables|Default|GetTraceEndLocation))
  (bind _returnvalue (Transformation|GetActorLocation _fromnode))
  (bind _returnvalue_2 (- _traceendlocation _returnvalue))
  (if (Variables|Default|GetIsPlacing)
    _
    (else
      (Rendering|SetVisibility (Variables|Default|GetPlacementWire) true false)
      (Rendering|SetVisibility (Variables|Default|GetWireNode) true false)
      (Variables|Default|SetIsPlacing true)))
  (Transformation|SetWorldLocationAndRotation (Variables|Default|GetPlacementWire) _returnvalue (Math|Conversions|RotationFromXVector _returnvalue_2) false true)
  (Transformation|SetRelativeScale3D (Variables|Default|GetPlacementWire) (Math|Vector|MakeVector 1.0 1.0 (Math|Vector|VectorLength _returnvalue_2)))
  (Transformation|SetWorldLocationAndRotation (Variables|Default|GetWireNode) (Variables|Default|GetTraceEndLocation) (Math|Conversions|RotationFromXVector (Variables|Default|GetHitNormal)) false true))

(fn HidePlacementWire
  (Rendering|SetVisibility (Variables|Default|GetPlacementWire) false false)
  (Rendering|SetVisibility (Variables|Default|GetWireNode) false false))

(fn SetCanPlace
  (params (CanPlace :type Boolean))
  (bind _cantplacecolor (Variables|Default|GetCantPlaceColor))
  (bind _canplacecolor (Variables|Default|GetCanPlaceColor))
  (bind _returnvalue (select CanPlace _canplacecolor _cantplacecolor))
  (Variables|Default|SetCanPlace CanPlace)
  (Rendering|Material|SetVectorParameterValueonMaterials (Variables|Default|GetPlacementWire) "Color" _returnvalue)
  (Rendering|Material|SetVectorParameterValueonMaterials (Variables|Default|GetWireNode) "Color" _returnvalue))

(fn AsInteractive
  (params (Component :type Primitive%20Component%20Object%20Reference))
  (bind _asbp_part_interactive (Utilities|Casting|CastToBP_PartInteractive (Components|GetOwner Component)))
  (return _asbp_part_interactive))