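; BP_HandManager is a physics grab tool that drags simulating objects along with the player's camera aim while it exists.
; Each tick it traces from the camera, latching onto the first physics component hit and storing the local grab point, distance and original damping.
; It pulls that point toward the aim with impulses scaled by squared distance and capped by mass, showing a debug arrow and mass.
; EndPlay restores the original damping.
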(event EventBeginPlay
  (Variables|Default|SetBuildRange (Math|Conversions|ToFloat(Integer) (Variables|/Game/FirstPersonBP/FirstPersonCharacter.FirstPersonCharacter_C|GetBuildRange (Variables|Default|GetPlayer)))))

(event EventEndPlay
  (params (EndPlayReason :type EEndPlayReason%20Enum :default "Destroyed"))
  (bind _hitcomponent (Variables|Default|GetHitComponent))
  (Utilities|IsValid _hitcomponent
    (:Is%20Valid
      (Class|PrimitiveComponent|SetLinearDamping _hitcomponent (Variables|Default|GetOriginalLinearDamping))
      (Class|PrimitiveComponent|SetAngularDamping _hitcomponent (Variables|Default|GetOriginalAngularDamping)))))

(event EventTick
  (params (DeltaSeconds :type Float%20%28single-precision%29))
  (bind _player (Variables|Default|GetPlayer))
  (bind _player_2 (Variables|Default|GetPlayer))
  (bind _firstpersoncamera (Variables|/Game/FirstPersonBP/FirstPersonCharacter.FirstPersonCharacter_C|GetFirstPersonCamera _player))
  (bind _returnvalue (Transformation|GetWorldLocation _firstpersoncamera))
  (bind (_outhit _returnvalue_2) (Collision|LineTraceByChannel _returnvalue (+ _returnvalue (* (Math|Vector|GetForwardVector _firstpersoncamera) (Variables|Default|GetBuildRange))) "TraceTypeQuery3" false (select (Utilities|IsValid (Variables|Default|GetHitComponent)) (Utilities|Array|MakeArray _player_2 (Variables|Default|GetHitActor)) (Utilities|Array|MakeArray _player_2)) "None"))
  (Utilities|IsValid (Variables|Default|GetHitComponent)
    (:Is%20Valid
      (Rendering|Debug|DrawDebugArrow (Math|Transform|TransformLocation (Transformation|GetWorldTransform (Variables|Default|GetHitComponent)) (Variables|Default|GetActorLocalHitLocation)) (Math|Vector|SelectVector (.Location (Collision|BreakHitResult _outhit)) (+ _returnvalue (* (Math|Vector|GetForwardVector _firstpersoncamera) (Variables|Default|GetBuildRange))) _returnvalue_2) 0.0 "(R=0.863157,G=0.225984,B=0.000000,A=1.000000)" 0.0 1.0)
      (Physics|AddImpulseatLocation (Variables|Default|GetHitComponent) (* (Math|Vector|Normalize (- (Math|Vector|SelectVector (.Location (Collision|BreakHitResult _outhit)) (+ _returnvalue (* (Math|Vector|GetForwardVector _firstpersoncamera) (Variables|Default|GetBuildRange))) _returnvalue_2) (Math|Transform|TransformLocation (Transformation|GetWorldTransform (Variables|Default|GetHitComponent)) (Variables|Default|GetActorLocalHitLocation)))) (Math|Float|Clamp(Float) (* (* (Math|Vector|VectorLength (- (Math|Vector|SelectVector (.Location (Collision|BreakHitResult _outhit)) (+ _returnvalue (* (Math|Vector|GetForwardVector _firstpersoncamera) (Variables|Default|GetBuildRange))) _returnvalue_2) (Math|Transform|TransformLocation (Transformation|GetWorldTransform (Variables|Default|GetHitComponent)) (Variables|Default|GetActorLocalHitLocation)))) (Math|Vector|VectorLength (- (Math|Vector|SelectVector (.Location (Collision|BreakHitResult _outhit)) (+ _returnvalue (* (Math|Vector|GetForwardVector _firstpersoncamera) (Variables|Default|GetBuildRange))) _returnvalue_2) (Math|Transform|TransformLocation (Transformation|GetWorldTransform (Variables|Default|GetHitComponent)) (Variables|Default|GetActorLocalHitLocation))))) 1.25) 0.0 (* (Physics|GetMass (Variables|Default|GetHitComponent)) 1e+02))) (Math|Transform|TransformLocation (Transformation|GetWorldTransform (Variables|Default|GetHitComponent)) (Variables|Default|GetActorLocalHitLocation)) "None")
      (CallFunction|PrintMass))
    (:Is%20Not%20Valid
      (if _returnvalue_2
        (if (Physics|IsSimulatingPhysics (.HitComponent (Collision|BreakHitResult _outhit)) "None")
          (Variables|Default|SetHitActor (.HitActor (Collision|BreakHitResult _outhit)))
          (bind _output_get (Variables|Default|SetHitComponent (.HitComponent (Collision|BreakHitResult _outhit))))
          (Variables|Default|SetActorLocalHitLocation (Math|Transform|InverseTransformLocation (Transformation|GetWorldTransform (.HitComponent (Collision|BreakHitResult _outhit))) (.Location (Collision|BreakHitResult _outhit))))
          (Variables|Default|SetBuildRange (Math|Vector|VectorLength (- (.Location (Collision|BreakHitResult _outhit)) (Transformation|GetWorldLocation (Variables|/Game/FirstPersonBP/FirstPersonCharacter.FirstPersonCharacter_C|GetFirstPersonCamera (Variables|Default|GetPlayer))))))
          (Variables|Default|SetOriginalLinearDamping (Class|PrimitiveComponent|GetLinearDamping _output_get))
          (Variables|Default|SetOriginalAngularDamping (Class|PrimitiveComponent|GetAngularDamping _output_get))
          (Class|PrimitiveComponent|SetLinearDamping _output_get (Variables|Default|GetLinearDamping))
          (Class|PrimitiveComponent|SetAngularDamping _output_get (Variables|Default|GetAngularDamping)))))))

(fn ConstructionScript)

(fn PrintMass
  (Development|PrintString (Utilities|String|Append "Mass: " (Utilities|String|ToString(Float) (Physics|GetMass (Variables|Default|GetHitComponent)))) true true "(R=1.000000,G=0.158568,B=0.369887,A=1.000000)" 0.0))