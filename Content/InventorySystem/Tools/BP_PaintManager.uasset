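; BP_PaintManager is the paint tool that recolors BP_Part actors the player aims at.
; Each action line-traces from the first-person camera out to the player's build range, keeping any BP_Part hit.
; Paint applies the player's paint color, UnPaint restores the base paint color, and SamplePaint copies the part's color to the player.
; Every trace draws a short-lived debug line from the gun in the current paint color.
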(event Custom|Paint
  (bind _hitpart (Variables|Default|GetHitPart))
  (CallFunction|UpdateTrace)
  (Utilities|IsValid _hitpart
    (:Is%20Valid
      (Default|SetColor _hitpart (Variables|/Game/FirstPersonBP/FirstPersonCharacter.FirstPersonCharacter_C|GetPaintColor (Variables|Default|GetPlayer))))))

(event Custom|UnPaint
  (bind _hitpart (Variables|Default|GetHitPart))
  (CallFunction|UpdateTrace)
  (Utilities|IsValid _hitpart
    (:Is%20Valid
      (Default|SetColor _hitpart (Variables|/Game/FirstPersonBP/FirstPersonCharacter.FirstPersonCharacter_C|GetPaintBaseColor (Variables|Default|GetPlayer))))))

(event Custom|SamplePaint
  (bind _hitpart (Variables|Default|GetHitPart))
  (CallFunction|UpdateTrace)
  (Utilities|IsValid _hitpart
    (:Is%20Valid
      (Variables|/Game/FirstPersonBP/FirstPersonCharacter.FirstPersonCharacter_C|SetPaintColor (Variables|Default|GetPlayer) (Variables|/Game/InventorySystem/Parts/BP_Part.BP_Part_C|GetPartColor _hitpart)))))

(fn ConstructionScript)

(fn UpdateTrace
  (bind _player (Variables|Default|GetPlayer))
  (bind _player_2 (Variables|Default|GetPlayer))
  (bind _firstpersoncamera (Variables|/Game/FirstPersonBP/FirstPersonCharacter.FirstPersonCharacter_C|GetFirstPersonCamera _player))
  (bind _paintcolor (Variables|/Game/FirstPersonBP/FirstPersonCharacter.FirstPersonCharacter_C|GetPaintColor _player_2))
  (bind (_x _y _z) (Math|Vector|BreakVector _paintcolor))
  (bind _returnvalue (Transformation|GetWorldLocation _firstpersoncamera))
  (bind (_outhit _returnvalue_2) (Collision|LineTraceByChannel _returnvalue (+ _returnvalue (* (Math|Vector|GetForwardVector _firstpersoncamera) (Variables|/Game/FirstPersonBP/FirstPersonCharacter.FirstPersonCharacter_C|GetBuildRange (Variables|Default|GetPlayer)))) "TraceTypeQuery1" false 0 "None"))
  (if _returnvalue_2
    (bind _asbp_part (Utilities|Casting|CastToBP_Part (.HitActor (Collision|BreakHitResult _outhit)))
      (:then
        (Variables|Default|SetHitPart _asbp_part))
      (:CastFailed
        (Variables|Default|SetHitPart 0 :!label _label)))
    (else
      (goto _label)))
  (Rendering|Debug|DrawDebugLine (Transformation|GetWorldLocation (Variables|/Game/FirstPersonBP/FirstPersonCharacter.FirstPersonCharacter_C|GetFP_Gun _player_2)) (.Location (Collision|BreakHitResult _outhit)) (Math|Color|MakeColor _x _y _z) 0.5 2.0))