(event Custom|Build
  (bind _placementnode (Variables|Default|GetPlacementNode))
  (CallFunction|AlignBuildPart)
  (if (Variables|Default|GetCanBuild)
    ;[1 1 1] Debug
    (Development|PrintString " - - - - - - - - - - - - - - - - - - - - - - - - - - - - - - - - - - - - BUILD" true true "(R=1.000000,G=1.000000,B=1.000000,A=1.000000)" 1e+02)
    (bind _returnvalue (Game|SpawnActorfromClass (Variables|/Game/FirstPersonBP/FirstPersonCharacter.FirstPersonCharacter_C|GetPartToBuild (Variables|Default|GetPlayer)) (Transformation|GetActorTransform (Variables|Default|GetActiveBuildPart)) "AlwaysSpawn" 0 false 0))
    (bind _output_get (Variables|Default|SetLastPlacedPart _returnvalue))
    (Variables|Default|SetLastPlacedComponent (Default|GetComponentbyTag _output_get (select (Components|ComponentHasTag _placementnode "Body0") "PartBody0" (select (Components|ComponentHasTag _placementnode "Body1") "PartBody1" (select (Components|ComponentHasTag _placementnode "Body2") "PartBody2" "PartBody3")))))
    (Default|SetColor _output_get (Variables|/Game/FirstPersonBP/FirstPersonCharacter.FirstPersonCharacter_C|GetPaintColor (Variables|Default|GetPlayer)))
    (if (Variables|/Game/FirstPersonBP/FirstPersonCharacter.FirstPersonCharacter_C|GetBuildLoose (Variables|Default|GetPlayer))
      (Default|InitBodies (Variables|Default|GetLastPlacedPart))
      (Development|PrintString "Build Loose" true true "(R=0.250000,G=0.415000,B=0.500000,A=1.000000)" 1e+02)
      (else
        (Utilities|IsValid (Variables|Default|GetLastHitPart)
          (:Is%20Valid
            (Development|PrintString "Placed on Part" true true "(R=0.250000,G=0.415000,B=0.500000,A=1.000000)" 1e+02)
            (Default|AttachtoPart (Variables|Default|GetLastPlacedPart) (Variables|Default|GetLastPlacedComponent) (Variables|Default|GetLastHitComponent)))
          (:Is%20Not%20Valid
            ;[1 1 1] Debug
            (Development|PrintString "Placed on world" true true "(R=0.250000,G=0.415000,B=0.500000,A=1.000000)" 1e+02)
            (Default|InitBodies (Variables|Default|GetLastPlacedPart))
            (Default|Ground (Variables|Default|GetLastPlacedPart) (Variables|Default|GetLastPlacedComponent))
            (Default|JoinStaticNeighbors (Variables|Default|GetLastPlacedPart) (Variables|Default|GetLastPlacedComponent))))))))

(event Custom|PrintHit
  ;[1 1 1] Debug
  (Utilities|IsValid (Variables|Default|GetLastHitPart)
    (:Is%20Valid
      (bind (_part _bodyindex _getbody _getpartcomponent _getattachcomp) (Default|GetREFs (Variables|Default|GetLastHitPart) (Variables|Default|GetLastHitComponent)))
      (Development|PrintString " - - - - - - - - - - - - - - - - - - - - - - - - - - - - - - - - - - - -" true true "(R=1.000000,G=0.016276,B=0.000000,A=1.000000)" 1e+02)
      (bind (_arrayindex _arrayelement) (Utilities|Array|ReverseforEachLoop (Variables|/Game/InventorySystem/Parts/BP_Body.BP_Body_C|GetMembers _getbody))
        (:LoopBody
          (Development|PrintString (Utilities|String|Append "Body Member " (Utilities|String|ToString(Integer) _arrayindex) " : " (Utilities|GetDisplayName _arrayelement)) true true "(R=0.000000,G=0.029118,B=0.546378,A=1.000000)" 1e+02))
        (:Completed
          (bind (_arrayindex_2 _arrayelement_2) (Utilities|Array|ReverseforEachLoop (Variables|/Game/InventorySystem/Parts/BP_Creation.BP_Creation_C|GetBodies (Variables|/Game/InventorySystem/Parts/BP_Part.BP_Part_C|GetCreation _part)))
            (:LoopBody
              (Development|PrintString (Utilities|String|Append "Creation Body " (Utilities|String|ToString(Integer) _arrayindex_2) " : " (Utilities|GetDisplayName _arrayelement_2)) true true "(R=0.700000,G=0.000000,B=0.241201,A=1.000000)" 1e+02))
            (:Completed
              (Development|PrintString (Utilities|String|Append "Body Creation: " (Utilities|GetObjectName (Variables|/Game/InventorySystem/Parts/BP_Body.BP_Body_C|GetCreation _getbody))) true true "(R=0.116971,G=0.009721,B=0.401978,A=1.000000)" 1e+02)
              (Development|PrintString (Utilities|String|Append "Part Creation: " (Utilities|GetObjectName (Variables|/Game/InventorySystem/Parts/BP_Part.BP_Part_C|GetCreation (Variables|Default|GetLastHitPart)))) true true "(R=0.116971,G=0.009721,B=0.401978,A=1.000000)" 1e+02)
              (Development|PrintString (Utilities|String|Append "Attached to: " (Utilities|GetDisplayName (Transformation|GetAttachParent _getattachcomp))) true true "(R=0.400000,G=0.000000,B=0.364252,A=1.000000)" 1e+02)
              (Development|PrintString (Utilities|String|Append "Body: " (Utilities|GetObjectName _getbody)) true true "(R=0.400000,G=0.000000,B=0.364252,A=1.000000)" 1e+02)
              (Development|PrintString (Utilities|String|Append "Simulating Physics: " (Utilities|String|ToString(Boolean) (Physics|IsSimulatingPhysics (Variables|Default|GetLastHitComponent) "None"))) true true "(R=0.400000,G=0.200000,B=0.382126,A=1.000000)" 1e+02)
              (Development|PrintString (Utilities|String|Append "Body Grounded: " (Utilities|String|ToString(Boolean) (Variables|/Game/InventorySystem/Parts/BP_Body.BP_Body_C|GetIsGrounded _getbody))) true true "(R=0.400000,G=0.200000,B=0.382126,A=1.000000)" 1e+02)
              (Development|PrintString (Utilities|String|Append "Part Grounded: " (Utilities|String|ToString(Boolean) (Variables|/Game/InventorySystem/Parts/BP_Part.BP_Part_C|GetIsGrounded (Variables|Default|GetLastHitPart)))) true true "(R=0.400000,G=0.200000,B=0.382126,A=1.000000)" 1e+02)
              (Development|PrintString (Utilities|String|Append "Component: " (Utilities|GetDisplayName (Variables|Default|GetLastHitComponent))) true true "(R=0.400000,G=0.000000,B=0.364251,A=1.000000)" 1e+02)
              (Development|PrintString (Utilities|String|Append "Actor: " (Utilities|GetDisplayName (Variables|Default|GetLastHitActor))) true true "(R=0.400000,G=0.000000,B=0.364252,A=1.000000)" 1e+02))))))))

(event Custom|SamplePart
  (bind _lasthitpart (Variables|Default|GetLastHitPart))
  (Utilities|IsValid _lasthitpart
    (:Is%20Valid
      (bind _asbp_part (Utilities|Casting|CastToBP_PartClass (Utilities|GetClass _lasthitpart)))
      (Variables|/Game/FirstPersonBP/FirstPersonCharacter.FirstPersonCharacter_C|SetPartToBuild (Variables|Default|GetPlayer) _asbp_part)
      (Utilities|IsValid (Variables|Default|GetActiveBuildPart)
        (:Is%20Valid
          (Actor|DestroyActor (Variables|Default|GetActiveBuildPart)))
        (:Is%20Not%20Valid
          _))
      (Variables|Default|SetActiveBuildPart 0))))

(event Custom|RemovePart
  (bind _lasthitpart (Variables|Default|GetLastHitPart))
  (Utilities|IsValid _lasthitpart
    (:Is%20Valid
      ;[1 1 1] Debug
      (Development|PrintString " - - - - - - - - - - - - - - - - - - - - - - - - - - - - - - - - - - - - DESTROY" true true "(R=1.000000,G=1.000000,B=1.000000,A=1.000000)" 1e+02)
      (Default|DestroyPart _lasthitpart 0 false))))

(event Custom|Update
  (bind _activebuildpart (Variables|Default|GetActiveBuildPart))
  (Utilities|IsValid _activebuildpart
    (:Is%20Valid
      (Actor|DestroyActor _activebuildpart))))

(event EventEndPlay
  (params (EndPlayReason :type EEndPlayReason%20Enum :default "Destroyed"))
  (Actor|DestroyActor (Variables|Default|GetActiveBuildPart)))

(event EventTick
  (params (DeltaSeconds :type Float%20%28single-precision%29))
  (Utilities|IsValid (Variables|Default|GetActiveBuildPart)
    (:Is%20Valid
      _)
    (:Is%20Not%20Valid
      (CallFunction|InitActivePart)))
  (Utilities|IsValid (Variables|Default|GetPlayer) ; In case player leaves while building
    (:Is%20Valid
      (CallFunction|AlignBuildPart))
    (:Is%20Not%20Valid
      (Actor|DestroyActor))))

(fn ConstructionScript)

(fn GetSnapLocation
  (params (HitLocation :type Vector) (HitNormal :type Vector))
  (bind _lasthitcomponent (Variables|Default|GetLastHitComponent))
  (bind _lasthitpart (Variables|Default|GetLastHitPart))
  (bind _returnvalue (Components|ComponentHasTag _lasthitcomponent "Body2"))
  (bind _returnvalue_2 (Components|ComponentHasTag _lasthitcomponent "Body0"))
  (bind _returnvalue_3 (Components|ComponentHasTag _lasthitcomponent "Body1"))
  (bind _returnvalue_4 (select _returnvalue "NodeBody2" "NodeBody3"))
  (bind _returnvalue_5 (select _returnvalue_3 "NodeBody1" _returnvalue_4))
  (bind _returnvalue_6 (select _returnvalue_2 "NodeBody0" _returnvalue_5))
  (bind _returnvalue_7 (Actor|GetComponentsbyTag _lasthitpart "/Script/Engine.PrimitiveComponent" _returnvalue_6))
  (if (> (Utilities|Array|Length _returnvalue_7) 0)
    (for (_array_element _array_index) _returnvalue_7
      (if (== _array_index 0)
        (LocalVariables|SetClosestDistance (Math|Vector|VectorLength (- HitLocation (.Location (Math|Transform|BreakTransform (Transformation|GetWorldTransform _array_element))))) :!label _label)
        (LocalVariables|SetClosestSnapLocation (.Location (Math|Transform|BreakTransform (Transformation|GetWorldTransform _array_element))))
        (LocalVariables|SetClosestSnapRotation (.Rotation (Math|Transform|BreakTransform (Transformation|GetWorldTransform _array_element))))
        (elif (< (Math|Vector|VectorLength (- HitLocation (.Location (Math|Transform|BreakTransform (Transformation|GetWorldTransform _array_element))))) (LocalVariables|GetClosestDistance))
          (goto _label))))
    (return (LocalVariables|GetClosestSnapLocation) (LocalVariables|GetClosestSnapRotation))
    (else
      (Variables|Default|SetCanBuild false)
      (LocalVariables|SetClosestSnapLocation HitLocation)
      (LocalVariables|SetClosestSnapRotation (Math|Rotator|MakeRotfromX HitNormal))
      (return (LocalVariables|GetClosestSnapLocation) (LocalVariables|GetClosestSnapRotation)))))

(fn ProcessRotationSet
  (params (Part :type BP%20Part%20Object%20Reference))
  (bind _returnvalue (Transformation|GetActorLocation Part))
  (if (>= (Variables|/Game/FirstPersonBP/FirstPersonCharacter.FirstPersonCharacter_C|GetBuildRotation1 (Variables|Default|GetPlayer)) (Variables|Default|GetRotationSetCount))
    (Variables|/Game/FirstPersonBP/FirstPersonCharacter.FirstPersonCharacter_C|SetBuildRotation1 (Variables|Default|GetPlayer) 0)
    (elif (< (Variables|/Game/FirstPersonBP/FirstPersonCharacter.FirstPersonCharacter_C|GetBuildRotation1 (Variables|Default|GetPlayer)) 0)
      (Variables|/Game/FirstPersonBP/FirstPersonCharacter.FirstPersonCharacter_C|SetBuildRotation1 (Variables|Default|GetPlayer) (- (Variables|Default|GetRotationSetCount) 1))))
  (if (>= (Variables|/Game/FirstPersonBP/FirstPersonCharacter.FirstPersonCharacter_C|GetBuildRotation3 (Variables|Default|GetPlayer)) (Utilities|Array|Length (Actor|GetComponentsbyTag Part "/Script/Engine.PrimitiveComponent" (Utilities|String|StringToName (Utilities|String|ToString(Integer) (Variables|/Game/FirstPersonBP/FirstPersonCharacter.FirstPersonCharacter_C|GetBuildRotation1 (Variables|Default|GetPlayer)))))))
    (Variables|/Game/FirstPersonBP/FirstPersonCharacter.FirstPersonCharacter_C|SetBuildRotation3 (Variables|Default|GetPlayer) 0)
    (elif (< (Variables|/Game/FirstPersonBP/FirstPersonCharacter.FirstPersonCharacter_C|GetBuildRotation3 (Variables|Default|GetPlayer)) 0)
      (Variables|/Game/FirstPersonBP/FirstPersonCharacter.FirstPersonCharacter_C|SetBuildRotation3 (Variables|Default|GetPlayer) (- (Utilities|Array|Length (Actor|GetComponentsbyTag Part "/Script/Engine.PrimitiveComponent" (Utilities|String|StringToName (Utilities|String|ToString(Integer) (Variables|/Game/FirstPersonBP/FirstPersonCharacter.FirstPersonCharacter_C|GetBuildRotation1 (Variables|Default|GetPlayer)))))) 1))))
  (Variables|Default|SetPlacementNode (Utilities|Array|Get(acopy) (Actor|GetComponentsbyTag Part "/Script/Engine.PrimitiveComponent" (Utilities|String|StringToName (Utilities|String|ToString(Integer) (Variables|/Game/FirstPersonBP/FirstPersonCharacter.FirstPersonCharacter_C|GetBuildRotation1 (Variables|Default|GetPlayer))))) (Variables|/Game/FirstPersonBP/FirstPersonCharacter.FirstPersonCharacter_C|GetBuildRotation3 (Variables|Default|GetPlayer))))
  (Transformation|AddActorLocalRotation Part (Utilities|Array|Get(acopy) (Variables|/Game/InventorySystem/Parts/BP_Part.BP_Part_C|GetRotationSet Part) (Variables|/Game/FirstPersonBP/FirstPersonCharacter.FirstPersonCharacter_C|GetBuildRotation1 (Variables|Default|GetPlayer))) false false)
  (Transformation|SetActorRotation Part (Math|Rotator|CombineRotators (Transformation|GetActorRotation Part) (Math|Vector|RotatorfromAxisandAngle (Math|Vector|GetForwardVector (Variables|Default|GetPlacementNode)) (* (Variables|/Game/FirstPersonBP/FirstPersonCharacter.FirstPersonCharacter_C|GetBuildRotation2 (Variables|Default|GetPlayer)) 9e+01))))
  (Transformation|SetActorLocation Part (- _returnvalue (- (Transformation|GetWorldLocation (Variables|Default|GetPlacementNode)) _returnvalue)) false false))

(fn InitActivePart
  (bind _returnvalue (Game|SpawnActorfromClass (Variables|/Game/FirstPersonBP/FirstPersonCharacter.FirstPersonCharacter_C|GetPartToBuild (Variables|Default|GetPlayer)) (Math|Transform|MakeTransform "0, 0, 0") "AlwaysSpawn" 0 true 0))
  (bind _output_get (Variables|Default|SetActiveBuildPart _returnvalue))
  (Collision|SetActorEnableCollision _output_get false)
  (Variables|Default|SetRotationSetCount (Utilities|Array|Length (Variables|/Game/InventorySystem/Parts/BP_Part.BP_Part_C|GetRotationSet _returnvalue)))
  (for _array_element (Actor|GetComponentsByClass _returnvalue "/Script/Engine.PrimitiveComponent")
    (Physics|SetSimulatePhysics _array_element false)
    (for _index (range 0 (- (Rendering|Material|GetNumMaterials _array_element) 1))
      (Rendering|Material|SetMaterial _array_element _index "/Game/Materials/M_Build_Inst.M_Build_Inst"))
    (if (!= _array_element (Variables|/Script/Engine.Actor|GetRootComponent _returnvalue))
      (Transformation|AttachComponentToComponent _array_element (Variables|/Script/Engine.Actor|GetRootComponent _returnvalue) "None" "KeepWorld" "KeepWorld" "KeepWorld" true))))

(fn CheckCanBuild
  (bind _activebuildpart (Variables|Default|GetActiveBuildPart))
  (bind _returnvalue (Actor|GetComponentsbyTag _activebuildpart "/Script/Engine.ActorComponent" "BuildCheck"))
  (if (Utilities|DoesObjectImplementInterface (Variables|Default|GetActiveBuildPart) "/Game/InventorySystem/Parts/Joints/JointInterface.JointInterface_C")
    (if (> (Utilities|Array|Length _returnvalue) 0)
      (bind _asprimitive_component (Utilities|Casting|CastToPrimitiveComponent (Utilities|Array|Get(acopy) _returnvalue))
        (:then
          (bind _outcomponents (Class|KismetSystemLibrary|ComponentOverlapComponents _asprimitive_component (Transformation|GetWorldTransform _asprimitive_component) (Utilities|Array|MakeArray "ObjectTypeQuery1" "ObjectTypeQuery2" "ObjectTypeQuery8") 0 (Utilities|Array|MakeArray (Variables|Default|GetActiveBuildPart))))
          (if (> (Utilities|Array|Length _outcomponents) 0)
            (Variables|Default|SetCanBuild false))
          (return (Variables|Default|GetCanBuild)))
        (:CastFailed
          _))))
  (return (Variables|Default|GetCanBuild)))

(fn PlacementTrace
  (bind _player (Variables|Default|GetPlayer))
  (bind _firstpersoncamera (Variables|/Game/FirstPersonBP/FirstPersonCharacter.FirstPersonCharacter_C|GetFirstPersonCamera _player))
  (bind _returnvalue (Transformation|GetWorldLocation _firstpersoncamera))
  (bind (_outhit _returnvalue_2) (Collision|LineTraceByChannel _returnvalue (+ _returnvalue (* (Math|Vector|GetForwardVector _firstpersoncamera) (Variables|/Game/FirstPersonBP/FirstPersonCharacter.FirstPersonCharacter_C|GetBuildRange (Variables|Default|GetPlayer)))) "TraceTypeQuery3" false (Utilities|Array|MakeArray (Variables|Default|GetActiveBuildPart) (Variables|Default|GetPlayer)) "None"))
  ;[1 1 1] Debug
  (Development|PrintString "____________________________________________________________" true true "(R=1.000000,G=1.000000,B=1.000000,A=1.000000)" 0.0)
  (bind _asbp_part (Utilities|Casting|CastToBP_Part (.HitActor (Collision|BreakHitResult _outhit)))
    (:then
      (bind (_part _bodyindex _getbody _getpartcomponent _getattachcomp) (Default|GetREFs _asbp_part (.HitComponent (Collision|BreakHitResult _outhit))))
      (Utilities|IsValid _getbody
        (:Is%20Valid
          (Development|PrintString (Utilities|String|Append "Body Creation: " (Utilities|GetObjectName (Variables|/Game/InventorySystem/Parts/BP_Body.BP_Body_C|GetCreation _getbody))) true true "(R=0.933092,G=0.552083,B=1.000000,A=1.000000)" 0.0)
          (Development|PrintString (Utilities|String|Append "Part Creation:  " (Utilities|GetObjectName (Variables|/Game/InventorySystem/Parts/BP_Part.BP_Part_C|GetCreation _part))) true true "(R=0.933092,G=0.552083,B=1.000000,A=1.000000)" 0.0)
          (Development|PrintString (Utilities|String|Append "Attch: " (Utilities|GetObjectName (Components|GetOwner (Transformation|GetAttachParent _getattachcomp)))) true true "(R=0.933092,G=0.552083,B=1.000000,A=1.000000)" 0.0)
          (Development|PrintString (Utilities|String|Append "Body: " (Utilities|GetObjectName _getbody)) true true "(R=0.933092,G=0.552083,B=1.000000,A=1.000000)" 0.0))
        (:Is%20Not%20Valid
          (Development|PrintString "..." true true "(R=0.933092,G=0.552083,B=1.000000,A=1.000000)" 0.0 :!label _label)
          (Development|PrintString "..." true true "(R=0.933092,G=0.552083,B=1.000000,A=1.000000)" 0.0)
          (Development|PrintString "..." true true "(R=0.933092,G=0.552083,B=1.000000,A=1.000000)" 0.0)
          (Development|PrintString "..." true true "(R=0.933092,G=0.552083,B=1.000000,A=1.000000)" 0.0))))
    (:CastFailed
      (goto _label)))
  (Development|PrintString (Utilities|String|Append "Comp Name: " (Utilities|GetObjectName (.HitComponent (Collision|BreakHitResult _outhit)))) true true "(R=0.933092,G=0.552083,B=1.000000,A=1.000000)" 0.0)
  (Development|PrintString (Utilities|String|Append "Actor Name:  " (Utilities|GetObjectName (.HitActor (Collision|BreakHitResult _outhit)))) true true "(R=0.933092,G=0.552083,B=1.000000,A=1.000000)" 0.0)
  (return _returnvalue_2 (.ImpactPoint (Collision|BreakHitResult _outhit)) (.ImpactNormal (Collision|BreakHitResult _outhit)) (.HitActor (Collision|BreakHitResult _outhit)) (.HitComponent (Collision|BreakHitResult _outhit))))

(fn AlignBuildPart
  (bind _activebuildpart (Variables|Default|GetActiveBuildPart))
  (bind _activebuildpart_2 (Variables|Default|GetActiveBuildPart))
  (bind _activebuildpart_3 (Variables|Default|GetActiveBuildPart))
  (bind (_hitsomething _hitlocation _hitnormal _hitactor _hitcomponent) (CallFunction|PlacementTrace))
  (if _hitsomething
    (Variables|Default|SetCanBuild true)
    (Variables|Default|SetLastHitActor _hitactor)
    (Variables|Default|SetLastHitComponent _hitcomponent)
    (Rendering|SetActorHiddenInGame _activebuildpart_2 false)
    (bind _asbp_part (Utilities|Casting|CastToBP_Part _hitactor) ; Was a Part hit?
      (:then
        (Variables|Default|SetLastHitPart _asbp_part)
        (bind (_snaplocation _snaprotation) (CallFunction|GetSnapLocation _hitlocation _hitnormal))
        (Transformation|SetActorLocationAndRotation _activebuildpart _snaplocation _snaprotation))
      (:CastFailed
        (Variables|Default|SetLastHitPart 0)
        (Transformation|SetActorLocationAndRotation _activebuildpart (Math|Vector|SelectVector (Math|Vector|MakeVector (* (Math|Float|Round (/ (.X (Math|Vector|BreakVector _hitlocation)) 2e+01)) 2e+01) (* (Math|Float|Round (/ (.Y (Math|Vector|BreakVector _hitlocation)) 2e+01)) 2e+01) (* (Math|Float|Floor (/ (.Z (Math|Vector|BreakVector _hitlocation)) 2e+01)) 2e+01)) _hitlocation (Variables|/Game/FirstPersonBP/FirstPersonCharacter.FirstPersonCharacter_C|GetBuildGridMode (Variables|Default|GetPlayer))) (Math|Rotator|SelectRotator "90.000000, 0, 0" (Math|Rotator|MakeRotator 0.0 9e+01 (.Yaw (Math|Rotator|BreakRotator (Transformation|GetWorldRotation (Variables|/Script/Engine.Character|GetCapsuleComponent (Variables|Default|GetPlayer)))))) (Variables|/Game/FirstPersonBP/FirstPersonCharacter.FirstPersonCharacter_C|GetBuildGridMode (Variables|Default|GetPlayer))))))
    (CallFunction|ProcessRotationSet _activebuildpart)
    (bind _canbuild (CallFunction|CheckCanBuild))
    (if _canbuild
      (if (Variables|/Game/FirstPersonBP/FirstPersonCharacter.FirstPersonCharacter_C|GetBuildLoose (Variables|Default|GetPlayer))
        (Default|SetColor _activebuildpart_3 "0,0.400000,1.000000") ; Build Loose
        (else
          (Default|SetColor _activebuildpart_3 "0,1.000000,0.000000") ; Can Build
        ))
      (else
        (Default|SetColor _activebuildpart_3 "1.000000,0.000000,0.000000") ; Cant Build
      ))
    (else
      (Variables|Default|SetCanBuild false)
      (Variables|Default|SetLastHitActor 0)
      (Variables|Default|SetLastHitComponent 0)
      (Rendering|SetActorHiddenInGame _activebuildpart_2 true))))

(fn AsPart
  (params (Component :type Primitive%20Component%20Object%20Reference))
  (bind _asbp_part (Utilities|Casting|CastToBP_Part (Components|GetOwner Component)))
  (return _asbp_part))